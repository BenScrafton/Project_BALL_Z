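; BP_GameMode_UI is a game mode that runs endless enemy waves of rising difficulty.
; Each new wave scales enemy count and spawn rate by a multiplier, then a looping timer spawns BP_Enemy at random TargetPoints until the count runs out.
; RegisterEnemyDeath removes enemies from the tracked array and, once none remain alive or pending, starts the next wave after a short delay.
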(event Custom|SpawnWave
  (CallFunction|SpawnEnemy))

(event Custom|EndWave
  (Utilities|FlowControl|Delay 2.0)
  (CallFunction|NewWaveSetup))

(event EventBeginPlay
  (Utilities|FlowControl|Delay 2.0)
  (CallFunction|NewWaveSetup))

(event EventTick
  (params (DeltaSeconds :type Float%20%28single-precision%29)))

(fn ConstructionScript)

(fn NewWaveSetup
  (Math|Integer|IncrementInt (Variables|Default|GetcurrentWave)
    (:%20%20
      (CallFunction|IncreaseWaveDifficulty)
      (Utilities|Time|SetTimerbyFunctionName 0 "SpawnWave" (Variables|Default|GetEnemySpawnFrequency) true))))

(fn SpawnEnemy
  (bind _spawnpoint (CallFunction|ChooseRandomSpawnPoint))
  (Utilities|IsValid _spawnpoint
    (:Is%20Valid
      (bind _returnvalue (Game|SpawnActorfromClass "/Game/Blueprints/AI/BP_Enemy.BP_Enemy_C" (Transformation|GetActorTransform _spawnpoint) "Undefined" 0 0))
      (Utilities|Array|Add (Variables|Default|Getenemies) _returnvalue)
      (bind _result (Math|Integer|DecrementInt (Variables|Default|GetenemySpawnsRemaining))
        (:%20%20
          (if (== _result 0)
            (Utilities|Time|ClearTimerbyFunctionName 0 "SpawnWave")))))))

(fn ChooseRandomSpawnPoint
  (bind _outactors (Actor|GetAllActorsOfClass "/Script/Engine.TargetPoint"))
  (return (Utilities|Array|Get(acopy) _outactors (Math|Random|RandomIntegerinRange 0 (Utilities|Array|LastIndex _outactors)))))

(fn RegisterEnemyDeath
  (params (enemy :type BP%20Enemy%20Object%20Reference%20%28by%20ref%29))
  (Utilities|Array|RemoveItem (Variables|Default|Getenemies) enemy)
  (if (CallFunction|IsWaveOver)
    (CallFunction|EndWave)))

(fn IsWaveOver
  (return (and (== (Variables|Default|GetenemySpawnsRemaining) 0) (== (Utilities|Array|Length (Variables|Default|Getenemies)) 0))))

(fn IncreaseWaveDifficulty
  (bind _output_get (Variables|Default|SetwaveDifficulty (Math|Float|Round (* (Variables|Default|GetwaveDifficulty) (Variables|Default|GetdifficultyMultiplier)))))
  (Variables|Default|SetenemySpawnsRemaining _output_get)
  (Variables|Default|SetEnemySpawnFrequency (/ (Variables|Default|GetEnemySpawnFrequency) (Variables|Default|GetdifficultyMultiplier))))