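; BP_WaterBucket is a thrown water bucket weapon prototype that damages on impact.
; BeginPlay loads durability and base damage from the weapons DataTable, then Throw pushes the mesh with an acceleration-change force and decrements durability.
; HitBox overlaps ignore weapons; enemy contact applies direct damage, while other contact triggers delayed, one-time radial damage excluding the player.
; Both impacts draw debug spheres and destroy the bucket shortly after.
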(event OnComponentBeginOverlap(HitBox)
  (params (OverlappedComponent :type Primitive%20Component%20Object%20Reference) (OtherActor :type Actor%20Object%20Reference) (OtherComp :type Primitive%20Component%20Object%20Reference) (OtherBodyIndex :type Integer) (bFromSweep :type Boolean) (SweepResult :type Hit%20Result%20Structure%20%28by%20ref%29))
  (bind _bucketmesh (Variables|Default|GetBucketMesh))
  (bind _returnvalue (Transformation|GetWorldLocation _bucketmesh))
  (if (not (Actor|ActorHasTag OtherActor "Weapon"))
    (if (Actor|ActorHasTag OtherActor "enemy")
      (Game|Damage|ApplyDamage 0 (Variables|Default|GetBase%20Weapon%20Damage) 0 0)
      (Rendering|Debug|DrawDebugSphere _returnvalue 1.5e+02 16 "(R=1.000000,G=0.000000,B=0.000000,A=1.000000)" 2.0 1.5)
      (Utilities|FlowControl|Delay 1.0)
      (Actor|DestroyActor)
      (else
        (Utilities|FlowControl|Delay 0.25)
        (Utilities|FlowControl|DoOnce false
          (:Completed
            (Rendering|Debug|DrawDebugSphere _returnvalue 1.5e+02 16 "(R=1.000000,G=0.000000,B=0.000000,A=1.000000)" 3.0 1.5)
            (Game|Damage|ApplyRadialDamage (Variables|Default|GetBase%20Weapon%20Damage) _returnvalue 1.5e+02 0 (Utilities|Array|MakeArray (Variables|Default|GetPlayer%20Ref)) self 0 false "ECC_Visibility")
            (Utilities|FlowControl|Delay 1.0)
            (Actor|DestroyActor)))))))

(event Custom|Throw
  (bind _bucketmesh (Variables|Default|GetBucketMesh))
  (bind _returnvalue (Math|Vector|GetForwardVector _bucketmesh))
  (bind (_x _y _z) (Math|Vector|BreakVector _returnvalue))
  (bind _returnvalue_2 (+ _z 3e+01))
  (bind _returnvalue_3 (+ _x 3e+01))
  (bind _returnvalue_4 (Math|Vector|MakeVector _returnvalue_3 _y _returnvalue_2))
  (bind _returnvalue_5 (* _returnvalue_4 2e+03))
  (bind (_x_2 _y_2 _z_2) (Math|Vector|BreakVector _returnvalue_5))
  (Development|PrintString (Utilities|String|ToString(Vector) (Math|Vector|MakeVector (Math|Float|Clamp(Float) _x_2 0.0 6.5e+04) _y_2 (Math|Float|Clamp(Float) _z_2 0.0 4.5e+04))))
  (Physics|AddForce (Variables|Default|GetBucketMesh) _returnvalue_5 "None" true)
  (CallFunction|DecrementDurability))

(event EventBeginPlay
  (|CallParentFunction)
  (Utilities|FlowControl|Sequence
    (:then_0
      (bind _returnvalue (Utilities|GetDataTableRow "/Game/A0051431-CF-Folder/DataTable/WeaponsDataTable.WeaponsDataTable" "Wep1B")
        (:then
          (Variables|Default|SetDurability (.Durability (Utilities|Struct|BreakWeaponsStructure _returnvalue)))
          (Variables|Default|SetBase%20Weapon%20Damage (.WeaponDamageBase (Utilities|Struct|BreakWeaponsStructure _returnvalue))))))
    (:then_1
      (CallFunction|Throw))))

(fn ConstructionScript
  (|CallParentFunction))