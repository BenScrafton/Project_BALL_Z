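; Base parent weapon Blueprint that handles melee-style damage and durability, caching the BP_Player pawn on BeginPlay.
; DamageEnemy applies base damage to actors tagged "enemy" only during the player's attack window, then plays a world camera shake and decrements durability.
; Durability drops per hit; a hit landing at zero calls WeaponDestroyed, which is empty here.
; Nothing in this Blueprint calls DamageEnemy.
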(event EventBeginPlay
  (bind _asbp_player (Utilities|Casting|CastToBP_Player (Game|Player|GetPlayerPawn 0)))
  (Variables|Default|SetPlayer%20Ref _asbp_player))

(fn ConstructionScript)

(fn DamageEnemy
  (params (EnemyActor :type Actor%20Object%20Reference))
  (if (Variables|/Game/Blueprints/Pawns/BP_Player.BP_Player_C|GetisInAttackWindow (Variables|Default|GetPlayer%20Ref))
    (if (Actor|ActorHasTag EnemyActor "enemy")
      (Game|Damage|ApplyDamage EnemyActor (Variables|Default|GetBase%20Weapon%20Damage) 0 0)
      (Development|PrintString "damage Success")
      (Camera|PlayWorldCameraShake "/Game/Blueprints/HitShake.HitShake_C" (Transformation|GetActorLocation) 0.0 1e+05)
      (CallFunction|DecrementDurability))))

(fn DecrementDurability
  (if (== (Variables|Default|GetDurability) 0)
    (CallFunction|WeaponDestroyed)
    (else
      (bind _result (Math|Integer|DecrementInt (Variables|Default|GetDurability))
        (:%20%20
          (Variables|Default|SetDurability _result))))))

(fn WeaponDestroyed)