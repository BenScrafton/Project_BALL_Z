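; BP_BaseWeapon_Mop is a prototype mop weapon that damages actors on contact and wears out with use.
; CollisionBox overlaps filter for actors tagged "None", then apply either ability or base damage depending on AbilityUsed.
; Each hit lowers Durability, and a hit at zero destroys the weapon, which a note flags for possible replacement with equipment detach logic.
; The short Delay after each decrement leads to no further logic.
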(event OnComponentBeginOverlap(Collisionbox)
  (params (OverlappedComponent :type Primitive%20Component%20Object%20Reference) (OtherActor :type Actor%20Object%20Reference) (OtherComp :type Primitive%20Component%20Object%20Reference) (OtherBodyIndex :type Integer) (bFromSweep :type Boolean) (SweepResult :type Hit%20Result%20Structure%20%28by%20ref%29))
  (if (Actor|ActorHasTag OtherActor "")
    (if (Variables|Default|GetAbility%20used%20?)
      (Game|Damage|ApplyDamage OtherActor (Variables|Default|GetDamage%20output%20%28ability%29) 0 0)
      (if (== (Variables|Default|GetDurability) 0)
        ;[1 1 1] May need to be replaced with event to detach and alter equipment assigned to player
        (Actor|DestroyActor)
        (else
          (Variables|Default|SetDurability (- (Variables|Default|GetDurability) 1))
          (Utilities|FlowControl|Delay 0.2)))
      (else
        (Game|Damage|ApplyDamage OtherActor (Variables|Default|GetDamage%20output%20%28Base%29) 0 0)
        (if (== (Variables|Default|GetDurability) 0)
          ;[1 1 1] same as above node
          (Actor|DestroyActor)
          (else
            (Variables|Default|SetDurability (- (Variables|Default|GetDurability) 1))
            (Utilities|FlowControl|Delay 0.2)))))))

(event EventBeginPlay
  (Variables|Default|SetDurability (Variables|Default|GetDurability)))

(fn ConstructionScript)