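; Prototype base melee weapon (mop test) that damages enemies it hits during the player's attack window.
; Caches the player pawn on BeginPlay, then on collision box overlap checks that window and the "enemy" tag before applying fixed damage and a world camera shake.
; An older ability/base damage branch with durability loss and self-destruction is disconnected and never runs, and DamageEnemy is an empty stub.
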(event OnComponentBeginOverlap(Collisionbox)
  (params (OverlappedComponent :type Primitive%20Component%20Object%20Reference) (OtherActor :type Actor%20Object%20Reference) (OtherComp :type Primitive%20Component%20Object%20Reference) (OtherBodyIndex :type Integer) (bFromSweep :type Boolean) (SweepResult :type Hit%20Result%20Structure%20%28by%20ref%29))
  (if (Variables|/Game/Blueprints/Pawns/BP_Player.BP_Player_C|GetisInAttackWindow (Variables|Default|Getplayer))
    (if (Actor|ActorHasTag OtherActor "enemy")
      (Game|Damage|ApplyDamage OtherActor 2e+01 0 0)
      (Camera|PlayWorldCameraShake "/Game/Blueprints/HitShake.HitShake_C" (Transformation|GetActorLocation) 0.0 1e+05))))

(event EventBeginPlay
  (bind _asbp_player (Utilities|Casting|CastToBP_Player (Game|Player|GetPlayerPawn 0)))
  (Variables|Default|Setplayer _asbp_player))

(event EventTick
  (params (DeltaSeconds :type Float%20%28single-precision%29)))

(fn ConstructionScript)

(fn DamageEnemy)