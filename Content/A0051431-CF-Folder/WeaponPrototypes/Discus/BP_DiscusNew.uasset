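; Thrown discus weapon that launches itself forward on BeginPlay, damaging enemies it passes through.
; BeginPlay loads durability and base damage from the weapons data table, then Throw applies a forward force and decrements durability.
; HitBox overlaps damage up to four enemies, briefly toggling each one's collision off, and destroy the discus on the next.
; Overlaps with other non-player, non-weapon actors add forward acceleration; debug prints remain.
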(event OnComponentHit(HitBox)
  (params (HitComponent :type Primitive%20Component%20Object%20Reference) (OtherActor :type Actor%20Object%20Reference) (OtherComp :type Primitive%20Component%20Object%20Reference) (NormalImpulse :type Vector :default "0, 0, 0") (Hit :type Hit%20Result%20Structure%20%28by%20ref%29)))

(event OnComponentBeginOverlap(HitBox)
  (params (OverlappedComponent :type Primitive%20Component%20Object%20Reference) (OtherActor :type Actor%20Object%20Reference) (OtherComp :type Primitive%20Component%20Object%20Reference) (OtherBodyIndex :type Integer) (bFromSweep :type Boolean) (SweepResult :type Hit%20Result%20Structure%20%28by%20ref%29))
  (bind _weaponmesh (Variables|Default|GetWeaponMesh))
  (bind _accelerator (Variables|Default|GetAccelerator))
  (bind _returnvalue (Math|Vector|GetForwardVector _weaponmesh))
  (bind _returnvalue_2 (* _returnvalue _accelerator))
  (if (not (Actor|ActorHasTag OtherActor "Weapon"))
    (if (Actor|ActorHasTag OtherActor "enemy")
      (if (< (Variables|Default|GetEnemy%20collisions) 4.0)
        (Development|PrintString (Utilities|String|ToString(Float) (Variables|Default|GetEnemy%20collisions)))
        (Game|Damage|ApplyDamage OtherActor (Variables|Default|GetBase%20Weapon%20Damage) 0 0)
        (Development|PrintString (Utilities|GetDisplayName OtherActor))
        (Variables|Default|SetEnemy%20collisions (+ (Variables|Default|GetEnemy%20collisions) 1.0))
        (Utilities|FlowControl|Sequence
          (:then_0
            (Collision|SetActorEnableCollision OtherActor false)
            (Utilities|FlowControl|Delay (.Time (Collision|BreakHitResult SweepResult)))
            (Collision|SetActorEnableCollision OtherActor true)))
        (else
          (Actor|DestroyActor)))
      (elif (not (Actor|ActorHasTag OtherActor "player"))
        (Physics|AddForce (Variables|Default|GetWeaponMesh) _returnvalue_2 "None" true)
        (Development|PrintString (Utilities|String|ToString(Vector) _returnvalue_2))))))

(event Custom|Throw
  (Physics|AddForce (Variables|Default|GetWeaponMesh) (* (Math|Vector|GetForwardVector (Variables|Default|GetWeaponMesh)) 1e+05) "None" true)
  (CallFunction|DecrementDurability))

(event EventBeginPlay
  (|CallParentFunction)
  (Utilities|FlowControl|Sequence
    (:then_0
      (bind _returnvalue (Utilities|GetDataTableRow "/Game/A0051431-CF-Folder/DataTable/WeaponsDataTable.WeaponsDataTable" "Wep1B")
        (:then
          (Variables|Default|SetDurability (.Durability (Utilities|Struct|BreakWeaponsStructure _returnvalue)))
          (Variables|Default|SetBase%20Weapon%20Damage (.WeaponDamageBase (Utilities|Struct|BreakWeaponsStructure _returnvalue))))))
    (:then_1
      (CallFunction|Throw))))

(fn ConstructionScript
  (|CallParentFunction))