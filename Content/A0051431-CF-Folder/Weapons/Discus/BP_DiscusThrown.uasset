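; Thrown discus projectile that launches with a forward force on spawn and takes its base damage from the weapons data table.
; Overlaps with weapons or walls add forward force, while players are ignored and a looping timer zeroes mesh rotation.
; It damages up to two enemies, briefly disabling their collision, and destroys itself after too many hits.
; If AbilityUsed is set on the second wall hit, it spends durability, spawns BP_DiscusAbilitySpawnPoint and destroys itself.
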(event OnComponentHit(HitBox)
  (params (HitComponent :type Primitive%20Component%20Object%20Reference) (OtherActor :type Actor%20Object%20Reference) (OtherComp :type Primitive%20Component%20Object%20Reference) (NormalImpulse :type Vector :default "0, 0, 0") (Hit :type Hit%20Result%20Structure%20%28by%20ref%29)))

(event OnComponentBeginOverlap(HitBox)
  (params (OverlappedComponent :type Primitive%20Component%20Object%20Reference) (OtherActor :type Actor%20Object%20Reference) (OtherComp :type Primitive%20Component%20Object%20Reference) (OtherBodyIndex :type Integer) (bFromSweep :type Boolean) (SweepResult :type Hit%20Result%20Structure%20%28by%20ref%29))
  (if (Actor|ActorHasTag OtherActor "Weapon")
    (Physics|AddForce (Variables|Default|GetWeaponMesh) (* (Math|Vector|GetForwardVector (Variables|Default|GetWeaponMesh)) (Variables|Default|GetAccelerator)) "None" true)
    (elif (Actor|ActorHasTag OtherActor "enemy")
      (if (< (Variables|Default|GetEnemy%20Collisions) 2.0)
        (Game|Damage|ApplyDamage OtherActor (Variables|Default|GetBase%20Weapon%20Damage) 0 0)
        (Development|PrintString (Utilities|GetDisplayName OtherActor))
        (Variables|Default|SetEnemy%20Collisions (+ (Variables|Default|GetEnemy%20Collisions) 1.0))
        (Utilities|FlowControl|Sequence
          (:then_0
            (Collision|SetActorEnableCollision OtherActor false)
            (Utilities|FlowControl|Delay (.Time (Collision|BreakHitResult SweepResult)))
            (Collision|SetActorEnableCollision OtherActor true)))
        (else
          (Actor|DestroyActor)))
      (elif (Actor|ActorHasTag OtherActor "player")
        (Collision|IgnoreActorwhenMoving (Variables|Default|GetHit%20Box) OtherActor true)
        (else
          (Physics|AddForce (Variables|Default|GetWeaponMesh) (* (Math|Vector|GetForwardVector (Variables|Default|GetWeaponMesh)) (Variables|Default|GetAccelerator)) "None" true)
          (if (< (Variables|Default|GetWall%20Collisions) 8.0)
            (Variables|Default|SetAbility%20Spawn%20point (Transformation|GetWorldLocation (Variables|Default|GetWeaponMesh)))
            (if (== (Variables|Default|GetWall%20Collisions) 1.0)
              (if (Variables|Default|GetAbility%20used%20?)
                (CallFunction|ABility)
                (Math|Float|IncrementFloat (Variables|Default|GetWall%20Collisions)
                  (:%20%20
                    (Variables|Default|SetAbility%20used%20? false)))
                (else
                  (Math|Float|IncrementFloat (Variables|Default|GetWall%20Collisions))))
              (else
                (Math|Float|IncrementFloat (Variables|Default|GetWall%20Collisions))))
            (else
              (Actor|DestroyActor))))))))

(event Custom|Throw
  (Physics|AddForce (Variables|Default|GetWeaponMesh) (* (Math|Vector|GetForwardVector (Variables|Default|GetWeaponMesh)) 1.25e+05) "None" true))

(event Custom|ABility
  (Utilities|FlowControl|Sequence
    (:then_0
      (Variables|Default|SetDurability (- (Variables|Default|GetDurability) 4))
      (Game|SpawnActorfromClass "/Game/A0051431-CF-Folder/Weapons/Discus/BP_DiscusAbilitySpawnPoint.BP_DiscusAbilitySpawnPoint_C" (Math|Transform|MakeTransform (Variables|Default|GetAbility%20Spawn%20point) (* (Transformation|GetWorldRotation (Variables|Default|GetWeaponMesh)) (Math|Random|RandomFloatinRange 0.5 1.0))) "Undefined" 0 0)
      (Utilities|FlowControl|Delay 0.2))
    (:then_1
      (Actor|DestroyActor))))

(event EventBeginPlay
  (|CallParentFunction)
  (bind _returnvalue (Utilities|GetDataTableRow "/Game/A0051431-CF-Folder/DataTable/WeaponsDataTable.WeaponsDataTable" "Wep3D")
    (:then
      (Variables|Default|SetBase%20Weapon%20Damage (.WeaponDamageBase (Utilities|Struct|BreakWeaponsStructure _returnvalue)))
      (Utilities|Time|SetTimerbyFunctionName 0 "Set Rotation" 0.01 true)
      (CallFunction|Throw))))

(fn ConstructionScript
  (|CallParentFunction))

(fn SetRotation
  (Transformation|SetWorldRotation (Variables|Default|GetWeaponMesh) "0, 0, 0" false false))