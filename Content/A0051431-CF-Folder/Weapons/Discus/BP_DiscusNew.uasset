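; Thrown discus weapon that flies toward the player's mouse location, with damage and durability read from the weapons data table.
; On attack it detaches, enables physics, re-equips a fresh discus on the player and launches, with a looping timer zeroing its rotation.
; Overlaps damage enemies or re-apply force, destroying it after capped enemy or wall hits.
; If AbilityUsed is set, the second wall hit spawns an ability spawn-point actor.
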(event OnComponentHit(HitBox)
  (params (HitComponent :type Primitive%20Component%20Object%20Reference) (OtherActor :type Actor%20Object%20Reference) (OtherComp :type Primitive%20Component%20Object%20Reference) (NormalImpulse :type Vector :default "0, 0, 0") (Hit :type Hit%20Result%20Structure%20%28by%20ref%29)))

(event OnComponentBeginOverlap(HitBox)
  (params (OverlappedComponent :type Primitive%20Component%20Object%20Reference) (OtherActor :type Actor%20Object%20Reference) (OtherComp :type Primitive%20Component%20Object%20Reference) (OtherBodyIndex :type Integer) (bFromSweep :type Boolean) (SweepResult :type Hit%20Result%20Structure%20%28by%20ref%29))
  (if (Actor|ActorHasTag OtherActor "Weapon")
    (Physics|AddForce (Variables|Default|GetWeaponMesh) (* (Math|Vector|GetForwardVector (Variables|Default|GetWeaponMesh)) (Variables|Default|GetAccelerator)) "None" true)
    (elif (Actor|ActorHasTag OtherActor "enemy")
      (if (< (Variables|Default|GetEnemy%20Collisions) 2.0)
        (Game|Damage|ApplyDamage OtherActor (Variables|Default|GetBase%20Weapon%20Damage) 0 0)
        (Development|PrintString (Utilities|GetDisplayName OtherActor))
        (Variables|Default|SetEnemy%20Collisions (+ (Variables|Default|GetEnemy%20Collisions) 1.0))
        (Utilities|FlowControl|Sequence
          (:then_0
            (Collision|SetActorEnableCollision OtherActor false)
            (Utilities|FlowControl|Delay (.Time (Collision|BreakHitResult SweepResult)))
            (Collision|SetActorEnableCollision OtherActor true)))
        (else
          (Variables|Default|SetIs%20destroyed%20? true)
          (CallFunction|DecrementDurability)
          (Actor|DestroyActor)))
      (elif (Actor|ActorHasTag OtherActor "player")
        (Collision|IgnoreActorwhenMoving (Variables|Default|GetHit%20Box) OtherActor true)
        (else
          (Physics|AddForce (Variables|Default|GetWeaponMesh) (* (Math|Vector|GetForwardVector (Variables|Default|GetWeaponMesh)) (Variables|Default|GetAccelerator)) "None" true)
          (if (< (Variables|Default|GetWall%20Collisions) 8.0)
            (Variables|Default|SetAbility%20Spawn%20point (Transformation|GetWorldLocation (Variables|Default|GetWeaponMesh)))
            (if (== (Variables|Default|GetWall%20Collisions) 1.0)
              (if (Variables|Default|GetAbility%20used%20?)
                (CallFunction|ABility)
                (Math|Float|IncrementFloat (Variables|Default|GetWall%20Collisions)
                  (:%20%20
                    (Variables|Default|SetAbility%20used%20? false)))
                (else
                  (Math|Float|IncrementFloat (Variables|Default|GetWall%20Collisions))))
              (else
                (Math|Float|IncrementFloat (Variables|Default|GetWall%20Collisions))))
            (else
              (Variables|Default|SetIs%20destroyed%20? true)
              (CallFunction|DecrementDurability)
              (Actor|DestroyActor))))))))

(event Custom|Throw
  (Variables|Default|SetIs%20destroyed%20? false)
  (Physics|AddForce (Variables|Default|GetWeaponMesh) (* (Math|Vector|GetForwardVector (Variables|Default|GetWeaponMesh)) 1e+05) "None" true)
  (CallFunction|DecrementDurability))

(event Custom|ABility
  (Utilities|FlowControl|Sequence
    (:then_0
      (Variables|Default|SetDurability (- (Variables|Default|GetDurability) 4))
      (Game|SpawnActorfromClass "/Game/A0051431-CF-Folder/Weapons/Discus/BP_DiscusAbilitySpawnPoint.BP_DiscusAbilitySpawnPoint_C" (Math|Transform|MakeTransform (Variables|Default|GetAbility%20Spawn%20point) (* (Transformation|GetWorldRotation (Variables|Default|GetWeaponMesh)) (Math|Random|RandomFloatinRange 0.5 1.0))) "Undefined" 0 0)
      (Utilities|FlowControl|Delay 0.2))
    (:then_1
      (Actor|DestroyActor))))

(event EventBeginPlay
  (|CallParentFunction)
  (Utilities|FlowControl|Sequence
    (:then_0
      (bind _returnvalue (Utilities|GetDataTableRow "/Game/A0051431-CF-Folder/DataTable/WeaponsDataTable.WeaponsDataTable" "Wep3D")
        (:then
          (Variables|Default|SetDurability (.Durability (Utilities|Struct|BreakWeaponsStructure _returnvalue)))
          (Variables|Default|SetBase%20Weapon%20Damage (.WeaponDamageBase (Utilities|Struct|BreakWeaponsStructure _returnvalue))))))
    (:then_1
      (Collision|SetCollisionEnabled (Variables|Default|GetHit%20Box) "NoCollision")
      (Variables|Default|SetIs%20destroyed%20? true))))

(event EventTick
  (params (DeltaSeconds :type Float%20%28single-precision%29))
  (Transformation|SetActorRelativeRotation "0, 0, 0"))

(fn ConstructionScript
  (|CallParentFunction))

(fn ExecuteAttack
  (|CallParentFunction)
  (if (Variables|Default|GetIs%20destroyed%20?)
    (Development|PrintString "Did it" true true "(R=1.000000,G=0.000000,B=0.079016,A=1.000000)")
    (Physics|SetSimulatePhysics (Variables|Default|GetWeaponMesh) true)
    (Collision|SetCollisionEnabled (Variables|Default|GetHit%20Box) "QueryAndPhysics")
    (Transformation|DetachFromActor "KeepWorld" "KeepWorld" "KeepWorld")
    (Variables|Default|SetIs%20destroyed%20? false)
    (bind _asbp_player (Utilities|Casting|CastToBP_Player (Game|GetPlayerCharacter 0)))
    (if (== (Variables|Default|GetDurability) 0)
      (CallFunction|WeaponDestroyed)
      (else
        (Default|EquipWeapon _asbp_player "BP_DiscusNew_C")
        (Physics|AddForce (Variables|Default|GetWeaponMesh) (* (Math|Vector|GetForwardVector (Math|Rotator|FindLookatRotation (Transformation|GetActorLocation _asbp_player) (Variables|/Game/Blueprints/Pawns/BP_Player.BP_Player_C|GetMouseLocation _asbp_player))) 1.5e+05) "None" true)
        (bind _returnvalue (Utilities|Time|SetTimerbyFunctionName 0 "Set Rotation" 0.001 true))
        (Variables|Default|SetRotation%20Handle _returnvalue)))))

(fn SetRotation
  (Transformation|SetWorldRotation (Variables|Default|GetWeaponMesh) "0, 0, 0" false false))