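; Blockout throwable discus weapon that flies along a direction vector and is meant to bounce off what it touches.
; Tick moves the actor with a swept world offset scaled by speed and delta time.
; HitBox overlap rotates the direction around Z by twice the angle to the impact normal to approximate a reflection, prints that angle, then pushes the mesh along the new direction.
; Throw and the hit event are empty.
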(event OnComponentHit(HitBox)
  (params (HitComponent :type Primitive%20Component%20Object%20Reference) (OtherActor :type Actor%20Object%20Reference) (OtherComp :type Primitive%20Component%20Object%20Reference) (NormalImpulse :type Vector :default "0, 0, 0") (Hit :type Hit%20Result%20Structure%20%28by%20ref%29)))

(event OnComponentBeginOverlap(HitBox)
  (params (OverlappedComponent :type Primitive%20Component%20Object%20Reference) (OtherActor :type Actor%20Object%20Reference) (OtherComp :type Primitive%20Component%20Object%20Reference) (OtherBodyIndex :type Integer) (bFromSweep :type Boolean) (SweepResult :type Hit%20Result%20Structure%20%28by%20ref%29))
  (Development|PrintString (Utilities|String|ToString(Float) (* 2 (CallFunction|FindAngleBetweenVectors (* (Variables|Default|Getdir%20Vector) -1.0) (.impactnormal SweepResult)))))
  (bind _output_get (Variables|Default|Setdir%20Vector (Math|Vector|RotateVectorAroundAxis (Variables|Default|Getdir%20Vector) (* 2 (CallFunction|FindAngleBetweenVectors (* (Variables|Default|Getdir%20Vector) -1.0) (.impactnormal SweepResult))) "0,0.000000,1.000000")))
  (Physics|AddForce (Variables|Default|GetWeaponMesh) _output_get "None" true))

(event Custom|Throw)

(event EventBeginPlay
  (|CallParentFunction))

(event EventTick
  (params (DeltaSeconds :type Float%20%28single-precision%29))
  (Transformation|AddActorWorldOffset (* (* (Variables|Default|Getdir%20Vector) (Variables|Default|Getspeed)) (Utilities|Time|GetWorldDeltaSeconds)) true))

(fn ConstructionScript
  (|CallParentFunction))