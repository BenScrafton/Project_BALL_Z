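; BP_DiscusAbilitySpawnPoint is a spawner actor for the discus ability that launches a set of three BP_AbilityDiscus actors.
; On BeginPlay, a DoOnce feeds a Sequence that spawns one discus at each of three Sphere components.
; Each discus takes the world location and rotation of its sphere at unit scale, so the component layout defines the spawn pattern.
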(event EventBeginPlay
  (bind _sphere (Variables|Default|GetSphere))
  (bind _sphere1 (Variables|Default|GetSphere1))
  (bind _sphere2 (Variables|Default|GetSphere2))
  (Utilities|FlowControl|DoOnce false
    (:Completed
      (Utilities|FlowControl|Sequence
        (:then_0
          (Game|SpawnActorfromClass "/Game/A0051431-CF-Folder/Weapons/Discus/BP_AbilityDiscus.BP_AbilityDiscus_C" (Math|Transform|MakeTransform (Transformation|GetWorldLocation _sphere) (Transformation|GetWorldRotation _sphere)) "Undefined" 0 0))
        (:then_1
          (Game|SpawnActorfromClass "/Game/A0051431-CF-Folder/Weapons/Discus/BP_AbilityDiscus.BP_AbilityDiscus_C" (Math|Transform|MakeTransform (Transformation|GetWorldLocation _sphere1) (Transformation|GetWorldRotation _sphere1) "1,1.000000,1") "Undefined" 0 0))
        (:then_2
          (Game|SpawnActorfromClass "/Game/A0051431-CF-Folder/Weapons/Discus/BP_AbilityDiscus.BP_AbilityDiscus_C" (Math|Transform|MakeTransform (Transformation|GetWorldLocation _sphere2) (Transformation|GetWorldRotation _sphere2)) "Undefined" 0 0))))))

(fn ConstructionScript)