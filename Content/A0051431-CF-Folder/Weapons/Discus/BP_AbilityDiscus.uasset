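; Thrown discus ability projectile that loads its stats from the weapons data table and launches itself forward on BeginPlay.
; HitBox overlaps damage tagged enemies, briefly disabling their collision, until an enemy hit limit destroys the discus.
; Weapon and other non-player overlaps re-apply forward force and count as wall collisions, with non-weapon overlaps destroying it at the limit.
; Reflection-vector bounce math is present but unused.
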(event OnComponentHit(HitBox)
  (params (HitComponent :type Primitive%20Component%20Object%20Reference) (OtherActor :type Actor%20Object%20Reference) (OtherComp :type Primitive%20Component%20Object%20Reference) (NormalImpulse :type Vector :default "0, 0, 0") (Hit :type Hit%20Result%20Structure%20%28by%20ref%29)))

(event OnComponentBeginOverlap(HitBox)
  (params (OverlappedComponent :type Primitive%20Component%20Object%20Reference) (OtherActor :type Actor%20Object%20Reference) (OtherComp :type Primitive%20Component%20Object%20Reference) (OtherBodyIndex :type Integer) (bFromSweep :type Boolean) (SweepResult :type Hit%20Result%20Structure%20%28by%20ref%29))
  (if (Actor|ActorHasTag OtherActor "Weapon")
    (Physics|AddForce (Variables|Default|GetWeaponMesh) (* (Math|Vector|GetForwardVector (Variables|Default|GetWeaponMesh)) (Variables|Default|GetAccelerator)) "None" true)
    (Math|Float|IncrementFloat (Variables|Default|GetWall%20Collisions))
    (elif (Actor|ActorHasTag OtherActor "enemy")
      (if (< (Variables|Default|GetEnemy%20Collisions) 4.0)
        (Game|Damage|ApplyDamage OtherActor (Variables|Default|GetAbility%20Damage) 0 0)
        (Development|PrintString (Utilities|GetDisplayName OtherActor))
        (Variables|Default|SetEnemy%20Collisions (+ (Variables|Default|GetEnemy%20Collisions) 1.0))
        (Utilities|FlowControl|Sequence
          (:then_0
            (Collision|SetActorEnableCollision OtherActor false)
            (Utilities|FlowControl|Delay (.Time (Collision|BreakHitResult SweepResult)))
            (Collision|SetActorEnableCollision OtherActor true)))
        (else
          (Variables|Default|SetIs%20destroyed%20? true)
          (Actor|DestroyActor)))
      (elif (not (Actor|ActorHasTag OtherActor "player"))
        (Physics|AddForce (Variables|Default|GetWeaponMesh) (* (Math|Vector|GetForwardVector (Variables|Default|GetWeaponMesh)) (Variables|Default|GetAccelerator)) "None" true)
        (if (< (Variables|Default|GetWall%20Collisions) 1e+01)
          (Math|Float|IncrementFloat (Variables|Default|GetWall%20Collisions))
          (else
            (Variables|Default|SetIs%20destroyed%20? true)
            (Actor|DestroyActor)))))))

(event Custom|Throw
  (Variables|Default|SetIs%20destroyed%20? false)
  (Physics|AddForce (Variables|Default|GetWeaponMesh) (* (Math|Vector|GetForwardVector (Variables|Default|GetWeaponMesh)) 1e+05) "None" true))

(event EventBeginPlay
  (Utilities|FlowControl|Sequence
    (:then_0
      (bind _returnvalue (Utilities|GetDataTableRow "/Game/A0051431-CF-Folder/DataTable/WeaponsDataTable.WeaponsDataTable" "Wep3D")
        (:then
          (Variables|Default|SetDurability (.Durability (Utilities|Struct|BreakWeaponsStructure _returnvalue)))
          (Variables|Default|SetBase%20Weapon%20Damage (.WeaponDamageBase (Utilities|Struct|BreakWeaponsStructure _returnvalue)))
          (Variables|Default|SetAbility%20Damage (.WeaponDamageAbility (Utilities|Struct|BreakWeaponsStructure _returnvalue))))))
    (:then_1
      (CallFunction|Throw))))

(fn ConstructionScript
  (|CallParentFunction))