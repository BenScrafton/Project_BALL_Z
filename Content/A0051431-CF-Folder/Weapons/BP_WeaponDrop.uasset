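; Weapon pickup that gives the player a random weapon from the weapons data table.
; On BeginPlay it picks a random row, applies that row's mesh and material, with a scale tweak for the Discus, and stores the weapon actor class.
; Tick spins it in yaw while a timeline bobs it vertically.
; Overlapping its box equips the weapon on a player with an empty weapon slot, then destroys the pickup.
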(event OnComponentBeginOverlap(PickupBox)
  (params (OverlappedComponent :type Primitive%20Component%20Object%20Reference) (OtherActor :type Actor%20Object%20Reference) (OtherComp :type Primitive%20Component%20Object%20Reference) (OtherBodyIndex :type Integer) (bFromSweep :type Boolean) (SweepResult :type Hit%20Result%20Structure%20%28by%20ref%29))
  (if (Actor|ActorHasTag OtherActor "player")
    (bind _asbp_player (Utilities|Casting|CastToBP_Player OtherActor))
    (if (== (Variables|/Game/Blueprints/Pawns/BP_Player.BP_Player_C|GetCurrent%20weapon%20Actor _asbp_player) 0)
      (Default|EquipWeapon _asbp_player (Variables|Default|GetActor))
      (Actor|DestroyActor))))

(event EventTick
  (params (DeltaSeconds :type Float%20%28single-precision%29))
  (bind _returnvalue (Transformation|GetActorRotation))
  (Transformation|SetWorldRotation (Variables|Default|GetDefaultSceneRoot) (Math|Rotator|MakeRotator (.roll _returnvalue) (.pitch _returnvalue) (+ (* DeltaSeconds 3e+02) (.yaw _returnvalue))) false false))

(event EventBeginPlay
  (bind _defaultsceneroot (Variables|Default|GetDefaultSceneRoot))
  (bind _weaponmesh (Variables|Default|GetWeaponMesh))
  (bind _returnvalue (Transformation|GetWorldLocation _defaultsceneroot))
  (Utilities|FlowControl|Sequence
    (:then_0
      (bind _movement (Timeline|Bob%20up%20and%20down Play)
        (:Update
          (Transformation|SetWorldLocation (Variables|Default|GetDefaultSceneRoot) (Math|Vector|MakeVector (.x _returnvalue) (.y _returnvalue) (+ _movement (.z _returnvalue))) false false))))
    (:then_1
      (bind _outrownames (DataTable|GetDataTableRowNames "/Game/A0051431-CF-Folder/DataTable/WeaponsDataTable.WeaponsDataTable"))
      (for _array_element _outrownames
        (Utilities|Array|Add (Variables|Default|GetRows%20) _array_element))
      (bind _returnvalue_2 (Utilities|GetDataTableRow "/Game/A0051431-CF-Folder/DataTable/WeaponsDataTable.WeaponsDataTable" (.OutItem (Utilities|Array|Random (Variables|Default|GetRows%20))))
        (:then
          (Components|StaticMesh|SetStaticMesh _weaponmesh (.Mesh (Utilities|Struct|BreakWeaponsStructure _returnvalue_2)))
          (if (== (.Mesh (Utilities|Struct|BreakWeaponsStructure _returnvalue_2)) "/Game/ArtAssets/Weapons/Discus/Discus.Discus")
            (Transformation|SetWorldScale3D (Variables|Default|GetWeaponMesh) "0.750000,0.750000,0.750000"))
          (Rendering|Material|SetMaterial _weaponmesh 0 (.MeshMaterial (Utilities|Struct|BreakWeaponsStructure _returnvalue_2)))
          (Variables|Default|SetActor (.Actor (Utilities|Struct|BreakWeaponsStructure _returnvalue_2))))))))

(fn ConstructionScript)