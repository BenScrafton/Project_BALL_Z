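; BP_CutleryKnife is a spinning cutlery knife weapon actor that damages enemies on contact.
; BeginPlay loads durability and damage from the Wep7C data table row, and Tick continuously spins the mesh.
; HitBox overlaps ignore player and weapon tags; enemies take random damage capped by AbilityDamage with a camera shake, while other hits randomise the knife's pitch.
; Either hit freezes the knife through zero time dilation, then destroys it after a delay.
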(event OnComponentBeginOverlap(StaticMesh)
  (params (OverlappedComponent :type Primitive%20Component%20Object%20Reference) (OtherActor :type Actor%20Object%20Reference) (OtherComp :type Primitive%20Component%20Object%20Reference) (OtherBodyIndex :type Integer) (bFromSweep :type Boolean) (SweepResult :type Hit%20Result%20Structure%20%28by%20ref%29)))

(event OnComponentBeginOverlap(HitBox)
  (params (OverlappedComponent :type Primitive%20Component%20Object%20Reference) (OtherActor :type Actor%20Object%20Reference) (OtherComp :type Primitive%20Component%20Object%20Reference) (OtherBodyIndex :type Integer) (bFromSweep :type Boolean) (SweepResult :type Hit%20Result%20Structure%20%28by%20ref%29))
  (bind _hitactor (Collision|BreakHitResult SweepResult))
  (if (not (Actor|ActorHasTag OtherActor "player"))
    (if (not (Actor|ActorHasTag OtherActor "Weapon"))
      (if (Actor|ActorHasTag _hitactor "enemy")
        (Utilities|FlowControl|DoOnce false
          (:Completed
            (Variables|Default|SetCustomTimeDilation 0.0)
            (Game|Damage|ApplyDamage _hitactor (Math|Random|RandomFloatinRange 1e+01 (Variables|Default|GetAbility%20Damage)) 0 0)
            (Camera|PlayWorldCameraShake "/Game/Blueprints/HitShake.HitShake_C" (Transformation|GetActorLocation) 0.0 1e+05)
            (Utilities|FlowControl|Delay 1.0)
            (Actor|DestroyActor)))
        (else
          (Transformation|SetRelativeRotation (Variables|Default|GetStaticMesh) (Math|Rotator|MakeRotator 0.0 (Math|Random|RandomFloatinRange -7e+01 -1e+02) 0.0) false false)
          (Variables|Default|SetCustomTimeDilation 0.0)
          (Utilities|FlowControl|Delay 1.0)
          (Actor|DestroyActor))))))

(event EventBeginPlay
  (|CallParentFunction)
  (bind _returnvalue (Utilities|GetDataTableRow "/Game/A0051431-CF-Folder/DataTable/WeaponsDataTable.WeaponsDataTable" "Wep7C")
    (:then
      (Variables|Default|SetDurability (.Durability (Utilities|Struct|BreakWeaponsStructure _returnvalue)))
      (Variables|Default|SetBase%20Weapon%20Damage (.WeaponDamageBase (Utilities|Struct|BreakWeaponsStructure _returnvalue)))
      (Variables|Default|SetAbility%20Damage (.WeaponDamageAbility (Utilities|Struct|BreakWeaponsStructure _returnvalue))))))

(event EventTick
  (params (DeltaSeconds :type Float%20%28single-precision%29))
  (Transformation|AddLocalRotation (Variables|Default|GetStaticMesh) (Math|Rotator|MakeRotator 0.0 (* DeltaSeconds -1.5e+03) 0.0) false false))

(fn ConstructionScript
  (|CallParentFunction))