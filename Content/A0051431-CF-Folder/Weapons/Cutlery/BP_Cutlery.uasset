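; BP_Cutlery is a weapon that throws a burst of cutlery as soon as it begins play, then decrements its durability.
; ThrowCutlery loops to spawn random classes from CutleryReferences around SpawnPoint with random X/Y jitter, with a Delay in the loop body.
; When AbilityUsed is set, Ability runs the same loop with BP_CutleryAbilityKnife instead.
; Both paths set ThrowCompleted after the loop.
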(event Custom|ThrowCutlery
  (bind _returnvalue (Math|Random|RandomFloatinRange -1e+02 1e+02))
  (bind _spawn_point (Variables|Default|GetSpawn%20point))
  (bind _returnvalue_2 (Transformation|GetWorldLocation _spawn_point))
  (if (Variables|Default|GetAbility%20used%20?)
    (CallFunction|Ability)
    (else
      (for _index (range 0 2)
        (Game|SpawnActorfromClass (.OutItem (Utilities|Array|Random (Variables|Default|GetCutlery%20References))) (Math|Transform|MakeTransform (Math|Vector|MakeVector (+ (.x _returnvalue_2) _returnvalue) (+ (.y _returnvalue_2) _returnvalue) (.z _returnvalue_2)) (Transformation|GetWorldRotation _spawn_point) "1,1,1") "AlwaysSpawn" 0 0)
        (Utilities|FlowControl|Delay 1.0))
      (Variables|Default|SetThrow%20completed%20? true))))

(event Custom|Ability
  (bind _returnvalue (Math|Random|RandomFloatinRange -1e+02 1e+02))
  (bind _spawn_point (Variables|Default|GetSpawn%20point))
  (bind _returnvalue_2 (Transformation|GetWorldLocation _spawn_point))
  (for _index (range 0 2)
    (Game|SpawnActorfromClass "/Game/A0051431-CF-Folder/Weapons/Cutlery/BP_CutleryAbilityKnife.BP_CutleryAbilityKnife_C" (Math|Transform|MakeTransform (Math|Vector|MakeVector (+ (.x _returnvalue_2) _returnvalue) (+ (.y _returnvalue_2) _returnvalue) (.z _returnvalue_2)) (Transformation|GetWorldRotation _spawn_point) "1,1,1") "AlwaysSpawn" 0 0)
    (Utilities|FlowControl|Delay 1.0))
  (Variables|Default|SetThrow%20completed%20? true))

(event EventBeginPlay
  (Utilities|FlowControl|Sequence
    (:then_0
      (CallFunction|ThrowCutlery)
      (Variables|Default|SetThrow%20completed%20? false))
    (:then_1
      (CallFunction|DecrementDurability))))

(fn ConstructionScript
  (|CallParentFunction))