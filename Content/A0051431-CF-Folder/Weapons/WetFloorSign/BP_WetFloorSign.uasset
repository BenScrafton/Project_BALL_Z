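; BP_WetFloorSign is a wet floor sign weapon Blueprint that damages enemies it touches.
; On BeginPlay it runs the parent logic, then loads durability, base damage and ability damage from its row in the weapons DataTable.
; HitBox overlaps call DamageEnemy with base damage on actors tagged "enemy", unless the weapon is flagged as detached.
; The AbilityUsed event is empty, so the loaded ability damage goes unused here.
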(event OnComponentBeginOverlap(HitBox)
  (params (OverlappedComponent :type Primitive%20Component%20Object%20Reference) (OtherActor :type Actor%20Object%20Reference) (OtherComp :type Primitive%20Component%20Object%20Reference) (OtherBodyIndex :type Integer) (bFromSweep :type Boolean) (SweepResult :type Hit%20Result%20Structure%20%28by%20ref%29))
  (if (not (Variables|Default|GetActor%20Detached%20?))
    (if (Actor|ActorHasTag OtherActor "enemy")
      (CallFunction|DamageEnemy OtherActor (Variables|Default|GetBase%20Weapon%20Damage)))))

(event Custom|Ability%20Used)

(event EventBeginPlay
  (|CallParentFunction)
  (bind _returnvalue (Utilities|GetDataTableRow "/Game/A0051431-CF-Folder/DataTable/WeaponsDataTable.WeaponsDataTable" "Wep6WFS")
    (:then
      (Variables|Default|SetDurability (.Durability (Utilities|Struct|BreakWeaponsStructure _returnvalue)))
      (Variables|Default|SetBase%20Weapon%20Damage (.WeaponDamageBase (Utilities|Struct|BreakWeaponsStructure _returnvalue)))
      (Variables|Default|SetAbility%20Damage (.WeaponDamageAbility (Utilities|Struct|BreakWeaponsStructure _returnvalue))))))

(fn ConstructionScript
  (|CallParentFunction))