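; BP_BroomStarterWeapon is a child broom weapon Blueprint that serves as the starter weapon.
; On BeginPlay it runs the parent logic, then sets durability to max int, making it effectively unbreakable, and sets its base damage.
; Hitbox overlaps pass the other actor and base damage to DamageEnemy.
; An Override Collision function hides the actor, disables hitbox collision and prints a debug message.
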(event OnComponentBeginOverlap(WeaponHitBox)
  (params (OverlappedComponent :type Primitive%20Component%20Object%20Reference) (OtherActor :type Actor%20Object%20Reference) (OtherComp :type Primitive%20Component%20Object%20Reference) (OtherBodyIndex :type Integer) (bFromSweep :type Boolean) (SweepResult :type Hit%20Result%20Structure%20%28by%20ref%29))
  (CallFunction|DamageEnemy OtherActor (Variables|Default|GetBase%20Weapon%20Damage)))

(event EventBeginPlay
  (|CallParentFunction)
  (Variables|Default|SetDurability 2147483647)
  (Variables|Default|SetBase%20Weapon%20Damage 35.0))

(fn ConstructionScript
  (|CallParentFunction))

(fn OverrideCollision
  (Rendering|SetActorHiddenInGame true)
  (Collision|SetCollisionEnabled (Variables|Default|GetWeaponHitBox) "NoCollision")
  (Development|PrintString "No collision"))