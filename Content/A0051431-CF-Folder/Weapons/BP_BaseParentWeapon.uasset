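; Base weapon Blueprint that handles melee damage, durability and breakage for the player's weapons.
; DamageEnemy hurts actors tagged "enemy" only during the player's attack window, then plays a camera shake and spends durability.
; On the last durability point, the equipped weapon detaches, launches forward as a physics object, and the player re-equips the starter broom.
; ExecuteAttack and OverrideCollision are empty here, and nothing in this file calls DamageEnemy.
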(event EventBeginPlay
  (bind _asbp_player (Utilities|Casting|CastToBP_Player (Game|Player|GetPlayerPawn 0)))
  (Variables|Default|SetPlayer%20Ref _asbp_player)
  (Variables|Default|SetActor%20Detached%20? false))

(fn ConstructionScript)

(fn DamageEnemy
  (params (EnemyActor :type Actor%20Object%20Reference) (Damage%20Input :type Float%20%28single-precision%29))
  (if (Variables|/Game/Blueprints/Pawns/BP_Player.BP_Player_C|GetisInAttackWindow (Variables|Default|GetPlayer%20Ref))
    (if (Actor|ActorHasTag EnemyActor "enemy")
      (Game|Damage|ApplyDamage EnemyActor Damage%20Input 0 0)
      (Camera|PlayWorldCameraShake "/Game/Blueprints/HitShake.HitShake_C" (Transformation|GetActorLocation) 0.0 1e+05)
      (CallFunction|DecrementDurability))))

(fn DecrementDurability
  (if (== (Variables|Default|GetDurability) 1)
    (CallFunction|WeaponDestroyed)
    (else
      (bind _result (Math|Integer|DecrementInt (Variables|Default|GetDurability))
        (:%20%20
          (Development|PrintString (Utilities|String|ToString(Integer) _result)))))))

(fn WeaponDestroyed
  (bind _player_ref (Variables|Default|GetPlayer%20Ref))
  (bind _skeletalmesh (Variables|Default|GetSkeletalMesh))
  (bind _asbp_player (Utilities|Casting|CastToBP_Player (Game|GetPlayerCharacter 0)))
  (Transformation|DetachFromActor (Variables|/Game/Blueprints/Pawns/BP_Player.BP_Player_C|GetCurrent%20weapon%20Actor (Variables|Default|GetPlayer%20Ref)) "KeepWorld" "KeepWorld" "KeepWorld")
  (Physics|SetSimulatePhysics _skeletalmesh true)
  (Physics|AddImpulse _skeletalmesh (* (Transformation|GetActorForwardVector _asbp_player) 5e+07) "None" true)
  (Variables|Default|SetActor%20Detached%20? true)
  (Variables|/Game/Blueprints/Pawns/BP_Player.BP_Player_C|SetWeaponAttached%20? _player_ref false)
  (Default|EquipWeapon _player_ref "/Game/A0051431-CF-Folder/Weapons/Broom/ChildBroomBP/BP_BroomStarterWeapon.BP_BroomStarterWeapon_C")
  (Variables|Default|SetBroom%20Attached%20? true))

(fn ExecuteAttack)

(fn OverrideCollision)