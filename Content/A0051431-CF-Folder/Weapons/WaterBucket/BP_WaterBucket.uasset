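; BP_WaterBucket is a weapon that throws a water bucket toward the player's mouse location.
; On BeginPlay it reads durability from the weapons data table, disables bucket collision and starts a looping timer that yaws an arrow toward the mouse.
; Each attack decrements durability, spawns a BP_WaterBucketThrown at the bucket with the arrow's yaw, and launches it toward the mouse by setting physics velocity.
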(event EventBeginPlay
  (|CallParentFunction)
  (Utilities|FlowControl|Sequence
    (:then_0
      (bind _returnvalue (Utilities|GetDataTableRow "/Game/A0051431-CF-Folder/DataTable/WeaponsDataTable.WeaponsDataTable" "Wep4WB")
        (:then
          (Variables|Default|SetDurability (.Durability (Utilities|Struct|BreakWeaponsStructure _returnvalue))))))
    (:then_1
      (Collision|SetCollisionEnabled (Variables|Default|GetBucketMesh) "NoCollision"))
    (:then_2
      (Utilities|Time|SetTimerbyFunctionName 0 "Face mouse" 0.005 true))
    (:then_3
      (bind _asbp_player (Utilities|Casting|CastToBP_Player (Game|Player|GetPlayerPawn 0)))
      (Variables|Default|SetAs%20BP%20Player _asbp_player))))

(fn ConstructionScript
  (|CallParentFunction))

(fn FaceMouse
  (bind _asbp_player (Utilities|Casting|CastToBP_Player (Game|Player|GetPlayerPawn 0)))
  (Transformation|SetWorldRotation (Variables|Default|GetArrow) (Math|Rotator|MakeRotator 0.0 0.0 (.yaw (Math|Rotator|FindLookatRotation (Transformation|GetWorldLocation (Variables|/Script/Engine.Character|GetMesh _asbp_player)) (Variables|/Game/Blueprints/Pawns/BP_Player.BP_Player_C|GetMouseLocation _asbp_player)))) false false))

(fn ExecuteAttack
  (|CallParentFunction)
  (CallFunction|DecrementDurability)
  (bind _returnvalue (Game|SpawnActorfromClass "/Game/A0051431-CF-Folder/Weapons/WaterBucket/BP_WaterBucketThrown.BP_WaterBucketThrown_C" (Math|Transform|MakeTransform (Transformation|GetWorldLocation (Variables|Default|GetBucketMesh)) (Math|Rotator|MakeRotator 0.0 0.0 (.yaw (Transformation|GetWorldRotation (Variables|Default|GetArrow)))) "1,1,1") "AlwaysSpawn" 0 0))
  (Physics|SetPhysicsLinearVelocity (Variables|/Game/A0051431-CF-Folder/Weapons/WaterBucket/BP_WaterBucketThrown.BP_WaterBucketThrown_C|GetBucketMesh _returnvalue) (* (Math|Vector|GetUnitDirection(Vector) (Transformation|GetActorLocation) (Variables|/Game/Blueprints/Pawns/BP_Player.BP_Player_C|GetMouseLocation (Variables|Default|GetAs%20BP%20Player))) 1.5e+03) false "None"))