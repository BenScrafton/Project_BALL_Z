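; BP_WaterBucketThrown is the thrown water bucket weapon actor, which damages the first enemy it hits.
; On BeginPlay it reads base damage from the weapons data table, then calls an empty Throw event.
; HitBox overlaps skip player and weapon actors; an enemy triggers damage once, spawns a water decal under the bucket, and destroys the actor after a delay.
; The launch-force and sphere-overlap debug nodes are disconnected.
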(event OnComponentBeginOverlap(HitBox)
  (params (OverlappedComponent :type Primitive%20Component%20Object%20Reference) (OtherActor :type Actor%20Object%20Reference) (OtherComp :type Primitive%20Component%20Object%20Reference) (OtherBodyIndex :type Integer) (bFromSweep :type Boolean) (SweepResult :type Hit%20Result%20Structure%20%28by%20ref%29))
  (bind _bucketmesh (Variables|Default|GetBucketMesh))
  (bind _returnvalue (Transformation|GetWorldLocation _bucketmesh))
  (if (not (Actor|ActorHasTag OtherActor "player"))
    (if (not (Actor|ActorHasTag OtherActor "Weapon"))
      (if (Actor|ActorHasTag OtherActor "enemy")
        (Utilities|FlowControl|DoOnce false
          (:Completed
            (Game|Damage|ApplyDamage OtherActor (Variables|Default|GetBase%20Weapon%20Damage) 0 0)
            (Game|SpawnActorfromClass "/Game/A0051431-CF-Folder/Weapons/WaterBucket/BP_WaterDecal.BP_WaterDecal_C" (Math|Transform|MakeTransform (Math|Vector|MakeVector (.x _returnvalue) (.y _returnvalue) 2e+01) "0, 0, 0" "0.300000,0.300000,0.300000") "Undefined" 0 0)
            (Utilities|FlowControl|Delay 1.0)
            (Actor|DestroyActor)))))))

(event Custom|Throw)

(event EventBeginPlay
  (|CallParentFunction)
  (Utilities|FlowControl|Sequence
    (:then_0
      (bind _returnvalue (Utilities|GetDataTableRow "/Game/A0051431-CF-Folder/DataTable/WeaponsDataTable.WeaponsDataTable" "Wep4WB")
        (:then
          (Variables|Default|SetBase%20Weapon%20Damage (.WeaponDamageBase (Utilities|Struct|BreakWeaponsStructure _returnvalue))))))
    (:then_1
      (CallFunction|Throw))))

(fn ConstructionScript
  (|CallParentFunction))