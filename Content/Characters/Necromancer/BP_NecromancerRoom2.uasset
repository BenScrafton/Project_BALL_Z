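; BP_NecromancerRoom2 is a scripted Necromancer appearance that triggers the Canteen room's enemy spawns and then leaves.
; On BeginPlay it snaps to a fixed rotation, waits TimeBeforeMove, then calls InitialEnemySpawns on BP_Default_GameMode.
; It then uses AI MoveTo toward RunPoint and destroys itself whether the move succeeds or fails.
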(event EventBeginPlay
  (Transformation|SetActorRotation "0,225.000000,0.000000")
  (Utilities|FlowControl|Delay (Variables|Default|GetTimeBeforeMove))
  (bind _asbp_default_game_mode (Utilities|Casting|CastToBP_Default_GameMode (Game|GetGameMode)))
  (Default|InitialEnemySpawns _asbp_default_game_mode "Canteen" true)
  (AI|AIMoveTo self (Variables|Default|GetRunPoint) 0 1.0 false
    (:OnSuccess
      (Actor|DestroyActor))
    (:OnFail
      (Actor|DestroyActor))))

(fn ConstructionScript)