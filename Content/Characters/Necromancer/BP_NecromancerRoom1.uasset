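; BP_NecromancerRoom1 is a scripted Necromancer that flees to a run point once it triggers enemy spawns in the room.
; After a delay on BeginPlay, it calls InitialEnemySpawns on the default game mode with the "Art" name, then AI-moves toward RunPoint.
; A lifespan timer starts as the move begins, and the actor also destroys itself when it reaches the point.
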(event EventBeginPlay
  (Utilities|FlowControl|Delay (Variables|Default|GetTimeBeforeMove))
  (bind _asbp_default_game_mode (Utilities|Casting|CastToBP_Default_GameMode (Game|GetGameMode)))
  (Default|InitialEnemySpawns _asbp_default_game_mode "Art")
  (AI|AIMoveTo self (Variables|Default|GetRunPoint) 0 0.0 false
    (:then
      (Actor|SetLifeSpan (Variables|Default|GetLifespan)))
    (:OnSuccess
      (Actor|DestroyActor))))

(fn ConstructionScript)