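; AI controller for a basketball AI that runs the BT_BasketBall behavior tree on BeginPlay.
; Every perception update writes the reported actor to the targetActor blackboard key, without checking whether it was sensed or lost.
; Tick polls InAttackRange and sets the inAttackRange key to true when it passes; this graph never resets it to false.
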(event OnTargetPerceptionUpdated(AIPerception)
  (params (Actor :type Actor%20Object%20Reference) (Stimulus :type AI%20Stimulus%20Structure))
  (AI|Components|Blackboard|SetValueasObject (Variables|Default|GetBlackboard) (Utilities|Name|MakeLiteralName "targetActor") Actor))

(event EventBeginPlay
  (|CallParentFunction)
  (AI|RunBehaviorTree "/Game/Blueprints/AI/BT_BasketBall.BT_BasketBall"))

(event EventTick
  (params (DeltaSeconds :type Float%20%28single-precision%29))
  (|CallParentFunction DeltaSeconds)
  (if (CallFunction|InAttackRange)
    (AI|Components|Blackboard|SetValueasBool (Variables|Default|GetBlackboard) (Utilities|Name|MakeLiteralName "inAttackRange") true)))

(fn ConstructionScript
  (|CallParentFunction))