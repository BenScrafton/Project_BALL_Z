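; BP_BasketBall is a bouncing enemy character that overrides movement, attack setup, damage and death from its AI parent.
; MoveToPlayer calls the parent with zero scale and hops when grounded.
; SetupAttack nudges it toward the player, leaping high when grounded and slamming down once horizontally close, while Attack itself is empty.
; Damage knocks it away from the player, and death enables capsule physics and launches it away.
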(event EventBeginPlay
  (|CallParentFunction))

(event EventTick
  (params (DeltaSeconds :type Float%20%28single-precision%29))
  (|CallParentFunction DeltaSeconds))

(fn ConstructionScript
  (|CallParentFunction))

(fn Kill
  (bind _returnvalue (Game|Player|GetPlayerPawn 0))
  (bind _returnvalue_2 (Transformation|GetActorLocation))
  (bind _returnvalue_3 (Transformation|GetActorLocation _returnvalue))
  (bind _returnvalue_4 (- _returnvalue_2 _returnvalue_3))
  (bind _returnvalue_5 (Math|Vector|Normalize _returnvalue_4))
  (bind _returnvalue_6 (* _returnvalue_5 2e+03))
  (Variables|Default|Sethealth 0.0)
  (Variables|Default|SetisDead true)
  (Development|PrintString ":(")
  (Physics|SetSimulatePhysics (Variables|Default|GetCapsuleComponent) true)
  (Physics|AddImpulse (Variables|Default|GetCapsuleComponent) (Math|Vector|MakeVector (.x _returnvalue_6) (.y _returnvalue_6) 0.0) "None" true))

(fn DecreaseHealth
  (params (damage :type Float%20%28single-precision%29))
  (bind _returnvalue (Game|Player|GetPlayerPawn 0))
  (bind _returnvalue_2 (Transformation|GetActorLocation))
  (bind _returnvalue_3 (Transformation|GetActorLocation _returnvalue))
  (bind _returnvalue_4 (- _returnvalue_2 _returnvalue_3))
  (bind _returnvalue_5 (Math|Vector|Normalize _returnvalue_4))
  (bind _returnvalue_6 (* _returnvalue_5 5e+02))
  (bind _health (|CallParentFunction damage))
  (Class|NavMovementComponent|StopActiveMovement (Variables|Character|GetCharacterMovement))
  (Physics|AddImpulse (Variables|Character|GetCharacterMovement) (Math|Vector|MakeVector (.x _returnvalue_6) (.y _returnvalue_6) 5e+01) true)
  (Development|PrintString "damage" true true "(R=1.000000,G=0.008603,B=0.000000,A=1.000000)")
  (return _health))

(fn Attack)

(fn MovetoPlayer
  (params (scale :type Float%20%28single-precision%29))
  (|CallParentFunction 0.0)
  (CallFunction|Bounce))

(fn Bounce
  (if (AI|Components|NavMovement|IsMovingonGround (Variables|Character|GetCharacterMovement))
    (Physics|AddImpulse (Variables|Character|GetCharacterMovement) "0, 0,500.000000" true)))

(fn SetupAttack
  (bind _returnvalue (Transformation|GetActorLocation))
  (bind _returnvalue_2 (Game|Player|GetPlayerPawn 0))
  (bind _returnvalue_3 (Transformation|GetActorLocation))
  (bind _returnvalue_4 (Game|Player|GetPlayerPawn 0))
  (bind _returnvalue_5 (Transformation|GetActorLocation _returnvalue_4))
  (bind _returnvalue_6 (Transformation|GetActorLocation _returnvalue_2))
  (bind _returnvalue_7 (- _returnvalue_6 _returnvalue_3))
  (bind _returnvalue_8 (Math|Vector|Normalize _returnvalue_7))
  (bind _returnvalue_9 (* _returnvalue_8 1e+01))
  (Transformation|AddActorLocalOffset (Math|Vector|MakeVector (.x _returnvalue_9) (.y _returnvalue_9) 0.0) false false)
  (if (< (Math|Vector|Distance(Vector) (Math|Vector|MakeVector (.x _returnvalue_5) (.y _returnvalue_5) 0.0) (Math|Vector|MakeVector (.x _returnvalue) (.y _returnvalue) 0.0)) 1e+02)
    (Physics|AddImpulse (Variables|Character|GetCharacterMovement) "0, 0,-1000.000000" true)
    (Development|PrintString "SLam")
    (elif (AI|Components|NavMovement|IsMovingonGround (Variables|Character|GetCharacterMovement))
      (Physics|AddImpulse (Variables|Character|GetCharacterMovement) "0, 0,1500.000000" true))))