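; BP_PaintRoller is an AI enemy that leaves paint streaks as it moves and knocks down the player on contact.
; Tick accumulates distance travelled and spawns a streak decal at DecalSpawnPoint whenever it reaches MoveDecalSpawnDist.
; Cylinder overlap damages BP_Player, launches them forward and upward, then calls KnockDown.
; Damage it receives is forwarded to its BP_AIEnemyController through ApplyDamage.
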(event OnComponentHit(Cylinder)
  (params (HitComponent :type Primitive%20Component%20Object%20Reference) (OtherActor :type Actor%20Object%20Reference) (OtherComp :type Primitive%20Component%20Object%20Reference) (NormalImpulse :type Vector :default "0, 0, 0") (Hit :type Hit%20Result%20Structure%20%28by%20ref%29)))

(event OnComponentBeginOverlap(Cylinder)
  (params (OverlappedComponent :type Primitive%20Component%20Object%20Reference) (OtherActor :type Actor%20Object%20Reference) (OtherComp :type Primitive%20Component%20Object%20Reference) (OtherBodyIndex :type Integer) (bFromSweep :type Boolean) (SweepResult :type Hit%20Result%20Structure%20%28by%20ref%29))
  (bind _returnvalue (Transformation|GetActorForwardVector))
  (bind _returnvalue_2 (* _returnvalue 2e+02))
  (bind _asbp_player (Utilities|Casting|CastToBP_Player OtherActor))
  (Development|PrintString "Hello")
  (Game|Damage|ApplyDamage _asbp_player 1e+01 0 0)
  (Physics|AddImpulse (Variables|/Script/Engine.Character|GetCharacterMovement _asbp_player) (Math|Vector|MakeVector (.x _returnvalue_2) (.y _returnvalue_2) 2e+02) true)
  (Default|KnockDown _asbp_player))

(event EventBeginPlay
  (Variables|Default|SetlastPos (Transformation|GetActorLocation)))

(event Collision|EventActorBeginOverlap
  (params (OtherActor :type Actor%20Object%20Reference)))

(event EventTick
  (params (DeltaSeconds :type Float%20%28single-precision%29))
  (bind _returnvalue (Transformation|GetActorLocation))
  (Variables|Default|SetcurMoveDistForDecal (+ (Variables|Default|GetcurMoveDistForDecal) (Math|Vector|Distance(Vector) _returnvalue (Variables|Default|GetlastPos))))
  (Variables|Default|SetlastPos _returnvalue)
  (if (>= (Variables|Default|GetcurMoveDistForDecal) (Variables|Default|GetmoveDecalSpawnDist))
    (Game|SpawnActorfromClass "/Game/Blueprints/AI/Enemies/PaintRoller/BP_paintStreakDecal.BP_paintStreakDecal_C" (Transformation|GetWorldTransform (Variables|Default|GetdecalSpawnPoint)) "Undefined" 0 0)
    (Variables|Default|SetcurMoveDistForDecal 0.0)))

(event Game|Damage|EventAnyDamage
  (params (Damage :type Float%20%28single-precision%29) (DamageType :type Damage%20Type%20Object%20Reference) (InstigatedBy :type Controller%20Object%20Reference) (DamageCauser :type Actor%20Object%20Reference))
  (bind _asbp_aienemy_controller (Utilities|Casting|CastToBP_AIEnemyController (Pawn|GetController)))
  (Game|Damage|ApplyDamage _asbp_aienemy_controller Damage 0 0))

(fn ConstructionScript)