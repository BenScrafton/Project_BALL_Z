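; American football enemy character that damages and knocks down the player on capsule contact, unless the player is dashing.
; Contact damage is armed only in one football state, polled from the AI blackboard each tick.
; A StunBP hit destroys that actor and disables movement for a few seconds.
; Received damage is forwarded to the BP_AIEnemyController with a hit sound, and overlaps with elite enemies trigger that controller's collision check.
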(event OnComponentBeginOverlap(CapsuleComponent)
  (params (OverlappedComponent :type Primitive%20Component%20Object%20Reference) (OtherActor :type Actor%20Object%20Reference) (OtherComp :type Primitive%20Component%20Object%20Reference) (OtherBodyIndex :type Integer) (bFromSweep :type Boolean) (SweepResult :type Hit%20Result%20Structure%20%28by%20ref%29))
  (if (Variables|Default|GetcanDamage)
    (bind _asbp_player (Utilities|Casting|CastToBP_Player OtherActor))
    (if (not (Variables|/Game/Blueprints/Pawns/BP_Player.BP_Player_C|GetIs%20Dashing _asbp_player))
      (Game|Damage|ApplyDamage _asbp_player 1e+01 0 0)
      (Default|KnockDown _asbp_player))))

(event Collision|EventHit
  (params (MyComp :type Primitive%20Component%20Object%20Reference) (Other :type Actor%20Object%20Reference) (OtherComp :type Primitive%20Component%20Object%20Reference) (bSelfMoved :type Boolean) (HitLocation :type Vector :default "0, 0, 0") (HitNormal :type Vector :default "0, 0, 0") (NormalImpulse :type Vector :default "0, 0, 0") (Hit :type Hit%20Result%20Structure%20%28by%20ref%29))
  (bind _asstun_bp (Utilities|Casting|CastToStunBP Other))
  (Actor|DestroyActor _asstun_bp)
  (Pawn|Components|CharacterMovement|DisableMovement (Variables|Character|GetCharacterMovement))
  (Utilities|FlowControl|Delay 7.0)
  (Pawn|Components|CharacterMovement|SetMovementMode (Variables|Character|GetCharacterMovement) "MOVE_Walking" 0))

(event Collision|EventActorBeginOverlap
  (params (OtherActor :type Actor%20Object%20Reference))
  (if (and (Actor|ActorHasTag OtherActor "enemy") (Actor|ActorHasTag OtherActor "Elite"))
    (bind _asbp_aienemy_controller (Utilities|Casting|CastToBP_AIEnemyController (Pawn|GetController)))
    (Default|EliteCollisionCheck _asbp_aienemy_controller)))

(event Game|Damage|EventAnyDamage
  (params (Damage :type Float%20%28single-precision%29) (DamageType :type Damage%20Type%20Object%20Reference) (InstigatedBy :type Controller%20Object%20Reference) (DamageCauser :type Actor%20Object%20Reference))
  (bind _asbp_aienemy_controller (Utilities|Casting|CastToBP_AIEnemyController (Pawn|GetController)))
  (Game|Damage|ApplyDamage _asbp_aienemy_controller Damage 0 0)
  (Audio|PlaySoundatLocation "/Game/Audio/Enemy_hit.Enemy_hit" "0, 0, 0" "0, 0, 0" 1.0 1.0 0.0 0 0 0))

(event EventTick
  (params (DeltaSeconds :type Float%20%28single-precision%29))
  (bind _output_get (Variables|Default|Setstate (Utilities|Enum|ByteToEnumEnum_FootballState (Class|BlackboardComponent|GetValueasEnum (AI|GetBlackboard (Pawn|GetController)) (Variables|Default|GetKey%20Name)))))
  (Variables|Default|SetcanDamage (Utilities|Enum|Equal(Enum) _output_get "NewEnumerator3")))

(event EventBeginPlay)

(event Collision|EventActorEndOverlap
  (params (OtherActor :type Actor%20Object%20Reference))
  (if (and (Actor|ActorHasTag OtherActor "enemy") (Actor|ActorHasTag OtherActor "Elite"))
    (bind _asbp_aienemy_controller (Utilities|Casting|CastToBP_AIEnemyController (Pawn|GetController)))
    (Default|EliteCollisionCheck _asbp_aienemy_controller)))

(fn ConstructionScript)