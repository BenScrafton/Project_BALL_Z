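; Enemy fruit actor that damages the player at close range.
; Each tick it checks the distance to player pawn 0 against an attack radius while it is allowed to hit.
; An attack applies damage, prints a debug string and plays a world camera shake, then blocks further hits until a cooldown timeline finishes.
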(event Custom|Attack
  (Development|PrintString "fruitHit")
  (Game|Damage|ApplyDamage (Variables|Default|GetPlayer) 1e+01 0 0)
  (Variables|Default|SetcanHit false)
  (Camera|PlayWorldCameraShake "/Game/Blueprints/HitShake.HitShake_C" (Transformation|GetActorLocation) 0.0 1e+05)
  (Timeline|AttackCooldown Play
    (:Finished
      (Variables|Default|SetcanHit true))))

(event EventBeginPlay
  (Variables|Default|SetPlayer (Game|Player|GetPlayerPawn 0)))

(event Collision|EventActorBeginOverlap
  (params (OtherActor :type Actor%20Object%20Reference)))

(event EventTick
  (params (DeltaSeconds :type Float%20%28single-precision%29))
  (if (and (Variables|Default|GetcanHit) (< (Math|Vector|Distance(Vector) (Transformation|GetActorLocation (Variables|Default|GetPlayer)) (Transformation|GetActorLocation)) (Variables|Default|GetattackRadius)))
    (CallFunction|Attack)))

(fn ConstructionScript)