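; BP_Tennisball is a tennis ball enemy character that hurts the player on contact and gets knocked back when damaged.
; When damaged under a BP_AIEnemyController, it launches up and away from the first player's pawn with a velocity-change impulse, then forwards the damage to that controller.
; Its sphere component's hit event applies a small fixed damage to BP_Player.
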(event OnComponentHit(Sphere)
  (params (HitComponent :type Primitive%20Component%20Object%20Reference) (OtherActor :type Actor%20Object%20Reference) (OtherComp :type Primitive%20Component%20Object%20Reference) (NormalImpulse :type Vector :default "0, 0, 0") (Hit :type Hit%20Result%20Structure%20%28by%20ref%29))
  (bind _asbp_player (Utilities|Casting|CastToBP_Player OtherActor))
  (Game|Damage|ApplyDamage _asbp_player 5.0 0 0))

(event Game|Damage|EventAnyDamage
  (params (Damage :type Float%20%28single-precision%29) (DamageType :type Damage%20Type%20Object%20Reference) (InstigatedBy :type Controller%20Object%20Reference) (DamageCauser :type Actor%20Object%20Reference))
  (bind _returnvalue (Game|Player|GetPlayerPawn 0))
  (bind _returnvalue_2 (Transformation|GetActorLocation))
  (bind _returnvalue_3 (Transformation|GetActorLocation _returnvalue))
  (bind _returnvalue_4 (- _returnvalue_2 _returnvalue_3))
  (bind _returnvalue_5 (Math|Vector|Normalize _returnvalue_4))
  (bind _returnvalue_6 (* _returnvalue_5 2e+03))
  (Development|PrintString "Tennisball Damage")
  (bind _asbp_aienemy_controller (Utilities|Casting|CastToBP_AIEnemyController (Pawn|GetController)))
  (Physics|AddImpulse (Variables|Character|GetCharacterMovement) (Math|Vector|MakeVector (.x _returnvalue_6) (.y _returnvalue_6) 1e+03) true)
  (Game|Damage|ApplyDamage _asbp_aienemy_controller Damage 0 0))

(fn ConstructionScript)