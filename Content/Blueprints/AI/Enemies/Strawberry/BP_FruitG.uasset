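; BP_FruitG is a strawberry melee enemy character that punches the player on a cooldown.
; Tick checks distance to the player, and Attack plays a punch montage, then applies delayed damage and a camera shake.
; Damage taken knocks it away from the player and is forwarded to its BP_AIEnemyController.
; Hits from StunBP actors destroy them and temporarily disable the enemy's movement.
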(event Custom|Attack
  (if (Variables|Default|GetcanHit)
    (Animation|Montage|PlayMontage (Variables|Default|GetStrawberry) "/Game/Blueprints/AI/Enemies/Strawberry/M_Punch.M_Punch" 3.0
      (:then
        (Utilities|FlowControl|Delay 0.2)
        (Game|Damage|ApplyDamage (Variables|Default|GetPlayer) 1e+01 0 0)
        (Variables|Default|SetcanHit false)
        (Camera|PlayWorldCameraShake "/Game/Blueprints/HitShake.HitShake_C" (Transformation|GetActorLocation) 0.0 1e+05)
        (Utilities|FlowControl|Delay 2.0)
        (Variables|Default|SetcanHit true)))))

(event Custom|CustomEvent
  (params (MyComp :type Primitive%20Component%20Object%20Reference) (Other :type Actor%20Object%20Reference) (OtherComp :type Primitive%20Component%20Object%20Reference) (bSelfMoved :type Boolean) (HitLocation :type Vector) (HitNormal :type Vector) (NormalImpulse :type Vector) (Hit :type Hit%20Result%20Structure%20%28by%20ref%29))
  (bind _asstun_bp (Utilities|Casting|CastToStunBP Other))
  (Actor|DestroyActor _asstun_bp)
  (Pawn|Components|CharacterMovement|DisableMovement (Variables|Character|GetCharacterMovement))
  (Utilities|FlowControl|Delay 7.0)
  (Pawn|Components|CharacterMovement|SetMovementMode (Variables|Character|GetCharacterMovement) "MOVE_Walking" 0))

(event EventTick
  (params (DeltaSeconds :type Float%20%28single-precision%29))
  (if (and (Variables|Default|GetcanHit) (< (Math|Vector|Distance(Vector) (Transformation|GetActorLocation (Variables|Default|GetPlayer)) (Transformation|GetActorLocation)) (Variables|Default|GetattackRadius)))
    (CallFunction|Attack)))

(event Game|Damage|EventAnyDamage
  (params (Damage :type Float%20%28single-precision%29) (DamageType :type Damage%20Type%20Object%20Reference) (InstigatedBy :type Controller%20Object%20Reference) (DamageCauser :type Actor%20Object%20Reference))
  (bind _returnvalue (Game|Player|GetPlayerPawn 0))
  (bind _returnvalue_2 (Transformation|GetActorLocation))
  (bind _returnvalue_3 (Transformation|GetActorLocation _returnvalue))
  (bind _returnvalue_4 (- _returnvalue_2 _returnvalue_3))
  (bind _returnvalue_5 (Math|Vector|Normalize _returnvalue_4))
  (bind _returnvalue_6 (* _returnvalue_5 5e+01))
  (bind _asbp_aienemy_controller (Utilities|Casting|CastToBP_AIEnemyController (Pawn|GetController)))
  (Transformation|AddActorWorldOffset (Math|Vector|MakeVector (.x _returnvalue_6) (.y _returnvalue_6) 0.0) true)
  (Game|Damage|ApplyDamage _asbp_aienemy_controller Damage 0 0)
  (Audio|PlaySoundatLocation "/Game/Audio/Enemy_hit.Enemy_hit" "0, 0, 0" "0, 0, 0" 1.0 1.0 0.0 0 0 0))

(event EventBeginPlay
  (Variables|Default|SetPlayer (Game|Player|GetPlayerPawn 0)))

(fn ConstructionScript)