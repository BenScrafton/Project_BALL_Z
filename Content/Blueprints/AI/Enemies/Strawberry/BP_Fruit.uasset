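; BP_Fruit is an enemy character that melee-attacks the player and can be stunned by StunBP actors.
; Tick checks distance to the cached player pawn and, within AttackRadius, applies damage with a camera shake.
; The AttackCooldown timeline gates repeat attacks by re-enabling CanHit when it finishes.
; A StunBP hit destroys that actor and disables movement for a fixed delay, but does not block attacks.
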(event Custom|Attack
  (Development|PrintString "fruitHit")
  (Variables|Default|SetHitting true)
  (Game|Damage|ApplyDamage (Variables|Default|GetPlayer) 1e+01 0 0)
  (Variables|Default|SetHitting false)
  (Variables|Default|SetcanHit false)
  (Camera|PlayWorldCameraShake "/Game/Blueprints/HitShake.HitShake_C" (Transformation|GetActorLocation) 0.0 1e+05)
  (Timeline|AttackCooldown Play
    (:Finished
      (Variables|Default|SetcanHit true))))

(event Collision|EventHit
  (params (MyComp :type Primitive%20Component%20Object%20Reference) (Other :type Actor%20Object%20Reference) (OtherComp :type Primitive%20Component%20Object%20Reference) (bSelfMoved :type Boolean) (HitLocation :type Vector :default "0, 0, 0") (HitNormal :type Vector :default "0, 0, 0") (NormalImpulse :type Vector :default "0, 0, 0") (Hit :type Hit%20Result%20Structure%20%28by%20ref%29))
  (bind _asstun_bp (Utilities|Casting|CastToStunBP Other))
  (Actor|DestroyActor _asstun_bp)
  (Pawn|Components|CharacterMovement|DisableMovement (Variables|Character|GetCharacterMovement))
  (Utilities|FlowControl|Delay 7.0)
  (Pawn|Components|CharacterMovement|SetMovementMode (Variables|Character|GetCharacterMovement) "MOVE_Walking" 0))

(event Collision|EventActorBeginOverlap
  (params (OtherActor :type Actor%20Object%20Reference)))

(event EventTick
  (params (DeltaSeconds :type Float%20%28single-precision%29))
  (if (and (Variables|Default|GetcanHit) (< (Math|Vector|Distance(Vector) (Transformation|GetActorLocation (Variables|Default|GetPlayer)) (Transformation|GetActorLocation)) (Variables|Default|GetattackRadius)))
    (CallFunction|Attack)))

(event EventBeginPlay
  (Variables|Default|SetPlayer (Game|Player|GetPlayerPawn 0)))

(fn ConstructionScript)