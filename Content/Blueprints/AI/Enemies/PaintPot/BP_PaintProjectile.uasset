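; Paint blob projectile of the PaintPot enemy, lobbed in an arc at the player's position sampled on BeginPlay.
; It solves initial vertical velocity from flight time and height difference, leaves vertical motion to BPCustomGravity, and sweeps horizontally each tick.
; On grounding it spawns a randomly rotated decal, plays a splat, applies radial damage and destroys itself.
; Overlapping the player attaches a separate paint decal actor to them.
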(event OnComponentBeginOverlap(Sphere)
  (params (OverlappedComponent :type Primitive%20Component%20Object%20Reference) (OtherActor :type Actor%20Object%20Reference) (OtherComp :type Primitive%20Component%20Object%20Reference) (OtherBodyIndex :type Integer) (bFromSweep :type Boolean) (SweepResult :type Hit%20Result%20Structure%20%28by%20ref%29))
  (bind _returnvalue (Game|Player|GetPlayerPawn 0))
  (if (== OtherActor _returnvalue)
    (bind _returnvalue_2 (Game|SpawnActorfromClass "/Game/Blueprints/AI/Enemies/PaintPot/BP_paintDecalForPlayerDown.BP_paintDecalForPlayerDown_C" (Math|Conversions|ToTransform(Vector) (Transformation|GetActorLocation _returnvalue)) "Undefined" 0 0))
    (Transformation|AttachActorToActor _returnvalue_2 _returnvalue "None" "SnapToTarget" "KeepRelative" "KeepWorld" true)))

(event EventBeginPlay
  (Utilities|IsValid (Game|Player|GetPlayerPawn 0)
    (:Is%20Valid
      (Variables|Default|SetTarget (Transformation|GetActorLocation (Game|Player|GetPlayerPawn 0)))
      (bind _time (CallFunction|CalculateTimetoApex))
      (CallFunction|CalculateInitVerticalVelocity _time)
      (CallFunction|CalculateDir))
    (:Is%20Not%20Valid
      (Actor|DestroyActor))))

(event EventTick
  (params (DeltaSeconds :type Float%20%28single-precision%29))
  (bind _bp_customgravity (Variables|Default|GetBP_CustomGravity))
  (bind _hitlocation (Variables|/Game/Blueprints/Components/BP_CustomGravity.BP_CustomGravity_C|GethitLocation _bp_customgravity))
  (if (not (Variables|/Game/Blueprints/Components/BP_CustomGravity.BP_CustomGravity_C|Getgrounded _bp_customgravity))
    (CallFunction|Move)
    (else
      (Game|SpawnActorfromClass "/Game/Blueprints/AI/Enemies/PaintPot/BP_paintDecal.BP_paintDecal_C" (Math|Transform|MakeTransform _hitlocation (Math|Rotator|MakeRotator 0.0 0.0 (Math|Random|RandomFloatinRange 0.0 3.6e+02)) "1,1,1") "Undefined" 0 0)
      (Audio|PlaySoundatLocation "/Game/Audio/Hamburger_splat.Hamburger_splat" "0, 0, 0" "0, 0, 0" 1.0 1.0 0.0 0 0 0)
      (Game|Damage|ApplyRadialDamage 1.0 _hitlocation 1e+02 0 0 0 0 false "ECC_Visibility")
      (Actor|DestroyActor))))

(fn ConstructionScript)

(fn CalculateTimetoApex
  (return (/ (Math|Vector|Distance(Vector) (Transformation|GetActorLocation) (Variables|Default|GetTarget)) (Variables|Default|GethorizontalSpeed))))

(fn CalculateInitVerticalVelocity
  (params (time :type Float%20%28single-precision%29))
  (bind _output_get (LocalVariables|SetverticalDisplacement (- (.z (Variables|Default|GetTarget)) (.z (Transformation|GetActorLocation)))))
  (Variables|/Game/Blueprints/Components/BP_CustomGravity.BP_CustomGravity_C|Setvelocity (Variables|Default|GetBP_CustomGravity) (Math|Vector|MakeVector 0.0 0.0 (/ (- _output_get (* 0.5 (* -1 (Variables|/Game/Blueprints/Components/BP_CustomGravity.BP_CustomGravity_C|GetGravityStrength (Variables|Default|GetBP_CustomGravity))) (* time time))) time))))

(fn Move
  (bind _returnvalue (Utilities|Time|GetWorldDeltaSeconds))
  (bind _dir (Variables|Default|Getdir))
  (bind _horizontalspeed (Variables|Default|GethorizontalSpeed))
  (bind _returnvalue_2 (* _horizontalspeed _returnvalue))
  (bind _returnvalue_3 (* _dir _returnvalue_2))
  (Transformation|AddActorWorldOffset (Math|Vector|MakeVector (.x _returnvalue_3) (.y _returnvalue_3) 0.0) true))

(fn CalculateDir
  (bind _returnvalue (Transformation|GetActorLocation))
  (bind _target (Variables|Default|GetTarget))
  (Variables|Default|Setdir (Math|Vector|Normalize (- (Math|Vector|MakeVector (.x _target) (.y _target) 0.0) (Math|Vector|MakeVector (.x _returnvalue) (.y _returnvalue) 0.0)))))