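; BP_PaintPot is an AI enemy that fires paint projectiles and hands its damage and Elite proximity events to its BP_AIEnemyController.
; Damage taken is re-applied to the controller actor through ApplyDamage.
; Begin and end overlaps with actors tagged both enemy and Elite trigger the controller's EliteCollisionCheck.
; LaunchProjectile spawns a BP_PaintProjectile at the ProjectileLaunchPoint transform.
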(event EventBeginPlay)

(event Collision|EventActorBeginOverlap
  (params (OtherActor :type Actor%20Object%20Reference))
  (if (and (Actor|ActorHasTag OtherActor "enemy") (Actor|ActorHasTag OtherActor "Elite"))
    (bind _asbp_aienemy_controller (Utilities|Casting|CastToBP_AIEnemyController (Pawn|GetController)))
    (Default|EliteCollisionCheck _asbp_aienemy_controller)))

(event Game|Damage|EventAnyDamage
  (params (Damage :type Float%20%28single-precision%29) (DamageType :type Damage%20Type%20Object%20Reference) (InstigatedBy :type Controller%20Object%20Reference) (DamageCauser :type Actor%20Object%20Reference))
  (bind _asbp_aienemy_controller (Utilities|Casting|CastToBP_AIEnemyController (Pawn|GetController)))
  (Game|Damage|ApplyDamage _asbp_aienemy_controller Damage 0 0))

(event EventTick
  (params (DeltaSeconds :type Float%20%28single-precision%29)))

(event Collision|EventActorEndOverlap
  (params (OtherActor :type Actor%20Object%20Reference))
  (if (and (Actor|ActorHasTag OtherActor "enemy") (Actor|ActorHasTag OtherActor "Elite"))
    (bind _asbp_aienemy_controller (Utilities|Casting|CastToBP_AIEnemyController (Pawn|GetController)))
    (Default|EliteCollisionCheck _asbp_aienemy_controller)))

(fn ConstructionScript)

(fn LaunchProjectile
  (Game|SpawnActorfromClass "/Game/Blueprints/AI/Enemies/PaintPot/BP_PaintProjectile.BP_PaintProjectile_C" (Transformation|GetWorldTransform (Variables|Default|GetProjectileLaunchPoint)) "Undefined" 0 0))