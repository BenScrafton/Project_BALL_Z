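; BP_Burger is an enemy character that leaps at targets, knocking down and hurting the player on overlap while CanDamage is set.
; ProcessJump solves a ballistic arc for BPCustomGravity from distance and horizontal speed, spawning an Attack_Indicator that grows over the calculated flight time.
; Move applies the horizontal travel.
; Damage is forwarded to the AI controller, and StunBP hits disable movement temporarily, restoring it as Walking rather than the initial Flying.
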(event OnComponentBeginOverlap(CapsuleComponent)
  (params (OverlappedComponent :type Primitive%20Component%20Object%20Reference) (OtherActor :type Actor%20Object%20Reference) (OtherComp :type Primitive%20Component%20Object%20Reference) (OtherBodyIndex :type Integer) (bFromSweep :type Boolean) (SweepResult :type Hit%20Result%20Structure%20%28by%20ref%29))
  (if (Variables|Default|GetcanDamage)
    (bind _asbp_player (Utilities|Casting|CastToBP_Player OtherActor))
    (Default|KnockDown _asbp_player)
    (Game|Damage|ApplyDamage _asbp_player 1e+01 0 0)))

(event Collision|EventHit
  (params (MyComp :type Primitive%20Component%20Object%20Reference) (Other :type Actor%20Object%20Reference) (OtherComp :type Primitive%20Component%20Object%20Reference) (bSelfMoved :type Boolean) (HitLocation :type Vector :default "0, 0, 0") (HitNormal :type Vector :default "0, 0, 0") (NormalImpulse :type Vector :default "0, 0, 0") (Hit :type Hit%20Result%20Structure%20%28by%20ref%29))
  (bind _asstun_bp (Utilities|Casting|CastToStunBP Other))
  (Actor|DestroyActor _asstun_bp)
  (Pawn|Components|CharacterMovement|DisableMovement (Variables|Character|GetCharacterMovement))
  (Utilities|FlowControl|Delay 7.0)
  (Pawn|Components|CharacterMovement|SetMovementMode (Variables|Character|GetCharacterMovement) "MOVE_Walking" 0))

(event Collision|EventActorBeginOverlap
  (params (OtherActor :type Actor%20Object%20Reference)))

(event EventTick
  (params (DeltaSeconds :type Float%20%28single-precision%29)))

(event Game|Damage|EventAnyDamage
  (params (Damage :type Float%20%28single-precision%29) (DamageType :type Damage%20Type%20Object%20Reference) (InstigatedBy :type Controller%20Object%20Reference) (DamageCauser :type Actor%20Object%20Reference))
  (Development|PrintString "Burger Damage")
  (bind _asbp_aienemy_controller (Utilities|Casting|CastToBP_AIEnemyController (Pawn|GetController)))
  (Game|Damage|ApplyDamage _asbp_aienemy_controller Damage 0 0)
  (Audio|PlaySoundatLocation "/Game/Audio/Enemy_hit.Enemy_hit" "0, 0, 0" "0, 0, 0" 1.0 1.0 0.0 0 0 0))

(event EventBeginPlay
  (Pawn|Components|CharacterMovement|SetMovementMode (Variables|Character|GetCharacterMovement) "MOVE_Flying" 0))

(fn ConstructionScript)

(fn ProcessJump
  (params (Target :type Vector))
  (Variables|/Game/Blueprints/Components/BP_CustomGravity.BP_CustomGravity_C|Setgrounded (Variables|Default|GetBP_CustomGravity) false)
  (Transformation|AddActorWorldOffset "0, 0,50.000000" false true)
  (Variables|Default|SetTarget Target)
  (bind _time (CallFunction|CalculateTimetoApex))
  (CallFunction|CalculateInitVerticalVelocity _time)
  (Game|SpawnActorfromClass "/Game/Blueprints/AI/Enemies/GolemBoss/Attack_Indicator.Attack_Indicator_C" (Math|Transform|MakeTransform (Math|Vector|MakeVector (.x (Variables|Default|GetTarget)) (.y (Variables|Default|GetTarget)) (- (.z (Variables|Default|GetTarget)) 1e+02)) "0, 0, 0" "1,1,1") "Undefined" 0 "0.500000,0.500000,0.500000" _time false 0)
  (CallFunction|CalculateDir))

(fn CalculateTimetoApex
  (return (/ (Math|Vector|Distance(Vector) (Transformation|GetActorLocation) (Variables|Default|GetTarget)) (Variables|Default|GethorizontalSpeed))))

(fn CalculateInitVerticalVelocity
  (params (time :type Float%20%28single-precision%29))
  (bind _output_get (LocalVariables|SetverticalDisplacement (- (.z (Variables|Default|GetTarget)) (.z (Transformation|GetActorLocation)))))
  (Variables|/Game/Blueprints/Components/BP_CustomGravity.BP_CustomGravity_C|Setvelocity (Variables|Default|GetBP_CustomGravity) (Math|Vector|MakeVector 0.0 0.0 (/ (- _output_get (* 0.5 (* -1 (Variables|/Game/Blueprints/Components/BP_CustomGravity.BP_CustomGravity_C|GetGravityStrength (Variables|Default|GetBP_CustomGravity))) (* time time))) time))))

(fn CalculateDir
  (bind _returnvalue (Transformation|GetActorLocation))
  (bind _target (Variables|Default|GetTarget))
  (Variables|Default|Setdir (Math|Vector|Normalize (- (Math|Vector|MakeVector (.x _target) (.y _target) 0.0) (Math|Vector|MakeVector (.x _returnvalue) (.y _returnvalue) 0.0)))))

(fn Move
  (Transformation|AddActorWorldOffset (* (Variables|Default|Getdir) (* (Variables|Default|GetHorizontalSpeed) (Utilities|Time|GetWorldDeltaSeconds))) true))