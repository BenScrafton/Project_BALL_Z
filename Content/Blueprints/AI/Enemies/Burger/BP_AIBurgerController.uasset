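; AI controller for the Burger enemy, which attacks by jumping at the player and then jumps away.
; A Tick-driven state machine cycles through cooldown, attack jump, travel, retreat jump to a random nearby navigable point, and travel back to cooldown.
; The pawn's custom gravity grounded flag ends each jump, and damage is enabled only during the airborne attack.
; A shared delta-time timer sets the grounded pauses before attacking and retreating.
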(event EventBeginPlay
  (|CallParentFunction)
  (bind _asbp_burger (Utilities|Casting|CastToBP_Burger (Pawn|GetControlledPawn)))
  (Variables|Default|Setburger _asbp_burger)
  (Default|ProcessJump (Variables|Default|Getburger) "0, 0, 0"))

(event EventTick
  (params (DeltaSeconds :type Float%20%28single-precision%29))
  (|CallParentFunction 0.0)
  (switch Utilities|FlowControl|Switch|SwitchonEnum_BurgerState (Variables|Default|Getstate)
    (:NewEnumerator2
      (if (Variables|/Game/Blueprints/Components/BP_CustomGravity.BP_CustomGravity_C|Getgrounded (Variables|/Game/Blueprints/AI/Enemies/Burger/BP_Burger.BP_Burger_C|GetBP_CustomGravity (Variables|Default|Getburger)))
        (bind _timeup (CallFunction|ProcessTimer))
        (if _timeup
          (Variables|Default|Setstate "NewEnumerator0")
          (CallFunction|RestartTimer))))
    (:NewEnumerator0
      (Default|ProcessJump (Variables|Default|Getburger) (Transformation|GetActorLocation (Game|Player|GetPlayerPawn 0)))
      (Variables|Default|Setstate "NewEnumerator1"))
    (:NewEnumerator1
      (if (Variables|/Game/Blueprints/Components/BP_CustomGravity.BP_CustomGravity_C|Getgrounded (Variables|/Game/Blueprints/AI/Enemies/Burger/BP_Burger.BP_Burger_C|GetBP_CustomGravity (Variables|Default|Getburger)))
        (bind _timeup_2 (CallFunction|ProcessTimer))
        (Variables|/Game/Blueprints/AI/Enemies/Burger/BP_Burger.BP_Burger_C|SetcanDamage (Variables|Default|Getburger) false)
        (if _timeup_2
          (CallFunction|RestartTimer)
          (Variables|Default|Setstate "NewEnumerator3"))
        (else
          (Default|Move (Variables|Default|Getburger))
          (Variables|/Game/Blueprints/AI/Enemies/Burger/BP_Burger.BP_Burger_C|SetcanDamage (Variables|Default|Getburger) true))))
    (:NewEnumerator3
      (Default|ProcessJump (Variables|Default|Getburger) (.RandomLocation (Class|NavigationSystemV1|GetRandomPointinNavigableRadius (Transformation|GetActorLocation (Variables|Default|Getburger)) 1e+03 0 0)))
      (Variables|Default|Setstate "NewEnumerator4"))
    (:NewEnumerator4
      (if (Variables|/Game/Blueprints/Components/BP_CustomGravity.BP_CustomGravity_C|Getgrounded (Variables|/Game/Blueprints/AI/Enemies/Burger/BP_Burger.BP_Burger_C|GetBP_CustomGravity (Variables|Default|Getburger)))
        (Variables|Default|Setstate "NewEnumerator2")
        (else
          (Default|Move (Variables|Default|Getburger)))))))

(fn ConstructionScript
  (|CallParentFunction))

(fn ProcessTimer
  (bind _output_get (Variables|Default|SetTimer (+ (Variables|Default|GetTimer) (Utilities|Time|GetWorldDeltaSeconds))))
  (if (> _output_get (Variables|Default|GetCooldownTime))
    _
    (else
      _))
  (return (> _output_get (Variables|Default|GetCooldownTime))))

(fn RestartTimer
  (Variables|Default|SetTimer 0.0))