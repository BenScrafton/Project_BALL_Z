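; Golem boss character for the Gym room: drops in on a spline, shows a health bar and enables the gym enemy spawn list.
; Health clamps at per-phase thresholds, flagging a Blackboard phase switch with invulnerability until the final death explosion.
; Slams follow a spline timeline, then spawn phase-scaled, randomly placed falling projectiles with indicators via looping DoN chains.
; Also handles spin and contact damage, plus temporary movement stuns from StunBP hits.
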(event OnComponentBeginOverlap(Cylinder)
  (params (OverlappedComponent :type Primitive%20Component%20Object%20Reference) (OtherActor :type Actor%20Object%20Reference) (OtherComp :type Primitive%20Component%20Object%20Reference) (OtherBodyIndex :type Integer) (bFromSweep :type Boolean) (SweepResult :type Hit%20Result%20Structure%20%28by%20ref%29))
  (if (Actor|ActorHasTag OtherActor "player")
    (Game|Damage|ApplyDamage OtherActor 1e+01 0 0)
    (Audio|PlaySoundatLocation "/Game/Audio/Enemy_hit.Enemy_hit" "0, 0, 0" "0, 0, 0" 1.0 1.0 0.0 0 0 0)))

(event Custom|Slam%20Attack%20Slam
  (params (Slam%20Time :type Float%20%28single-precision%29))
  (bind _returnvalue (Game|GetPlayerCharacter 0))
  (bind _spline_ref (Variables|Default|GetSpline%20Ref))
  (bind _returnvalue_2 (Transformation|GetActorLocation _returnvalue))
  (bind _spline (Variables|/Game/Blueprints/AI/Enemies/GolemBoss/SlamAttackSpline.SlamAttackSpline_C|GetSpline _spline_ref))
  (Utilities|FlowControl|DoOnce false
    (:Completed
      (Transformation|SetActorLocation (+ (Transformation|GetActorLocation (Game|GetPlayerCharacter 0)) "0, 0,2500.000000") false false)
      (bind _outhit (Collision|LineTraceForObjects _returnvalue_2 (- _returnvalue_2 "0, 0,250.000000") (Utilities|Array|MakeArray "ObjectTypeQuery1") false (Utilities|Array|MakeArray _returnvalue) "None"))
      (Game|SpawnActorfromClass "/Game/Blueprints/AI/Enemies/GolemBoss/Attack_Indicator.Attack_Indicator_C" (Math|Transform|MakeTransform (.Location (Collision|BreakHitResult _outhit)) "0, 0, 0" "1,1,1") "Undefined" 0 "2.000000,2.000000,2.000000" 2.0 true 0)
      (bind _spline_progress (Timeline|Slam PlayFromStart)
        (:Update
          (Transformation|SetActorLocation (Spline|GetLocationatDistanceAlongSpline _spline (* (Spline|GetSplineLength _spline) _spline_progress) "World") false false))
        (:Finished
          (Variables|/Script/Engine.MovementComponent|SetVelocity (Variables|Character|GetCharacterMovement) "0, 0, 0")
          (Actor|DestroyActor (Variables|Default|GetSpline%20Ref))
          (Camera|PlayWorldCameraShake "/Game/Blueprints/AI/Enemies/GolemBoss/GolemBossCameraShake.GolemBossCameraShake_C" (Transformation|GetWorldLocation (Variables|Default|GetCameraShakeSource)) 5e+03 5e+04)
          (Components|Activation|Activate (Variables|Default|GetRock%20Smash%20Particle) true)
          (Math|Integer|CompareInt (Variables|Default|GetPhase) 2
            (:>
              (CallFunction|BigSlamAttackFallingProjectiles :!label _label))
            (:==
              (goto _label))
            (:<
              _))
          (CallFunction|SmallSlamAttackFallingProjectiles)
          (Utilities|FlowControl|Delay 3.0)
          (CallFunction|SlamAttackReset)
          (Components|Activation|Deactivate (Variables|Default|GetRock%20Smash%20Particle)))
        (:Slam%20Animation%20Start
          (Components|Animation|PlayAnimation (Variables|Character|GetMesh) "/Game/Characters/Golum+Animations/Golum_LP_Anim_Gollum_Skeleton_0SlamAttackAnim2.Golum_LP_Anim_Gollum_Skeleton_0SlamAttackAnim2" false))))))

(event Custom|Slam%20Attack%20Reset
  (bind _returnvalue (Game|GetPlayerCharacter 0))
  (bind _spline_ref (Variables|Default|GetSpline%20Ref))
  (bind _returnvalue_2 (Transformation|GetActorLocation _returnvalue))
  (bind _spline (Variables|/Game/Blueprints/AI/Enemies/GolemBoss/SlamAttackSpline.SlamAttackSpline_C|GetSpline _spline_ref))
  (Utilities|FlowControl|DoOnce false) ; enters at Reset
)

(event Custom|Initial%20Phase%20Shift
  (Variables|Default|SetInitial%20Invulnerability false)
  (AI|Components|Blackboard|SetValueasBool (AI|GetBlackboard 0) (Utilities|Name|MakeLiteralName "Phase Switch") true)
  (Variables|Default|SetPhase%20Shifting true))

(event Custom|Damage%20Loop
  (bind _returnvalue (Game|Player|GetPlayerPawn 0))
  (if (and (Collision|IsOverlappingActor _returnvalue :!class /Script/Engine.Actor) (Variables|Default|GetSpin%20Attack))
    (Game|Damage|ApplyDamage _returnvalue 1.0 0 0))
  (Utilities|FlowControl|Delay 0.2)
  (CallFunction|DamageLoop))

(event Custom|Small%20Slam%20Attack%20Falling%20Projectiles
  (bind _slam_attack_boundary_1_location (Variables|Default|GetSlam%20Attack%20Boundary%201%20Location))
  (bind _slam_attack_boundary_2_location (Variables|Default|GetSlam%20Attack%20Boundary%202%20Location))
  (bind _phase (Variables|Default|GetPhase))
  (bind _returnvalue (Math|Conversions|ToFloat(Integer) _phase))
  (bind _returnvalue_2 (Math|Float|Power _returnvalue 1.5))
  (bind _returnvalue_3 (* 4 _returnvalue_2))
  (bind _returnvalue_4 (Math|Float|Ceil _returnvalue_3))
  (Utilities|FlowControl|Delay (Math|Random|RandomFloatinRange 0.3 (- 1.75 (* (Variables|Default|GetPhase) 0.5))))
  (Variables|Default|SetSmall%20Projectile%20Location (Math|Vector|MakeVector (Math|Random|RandomFloatinRange (.x _slam_attack_boundary_1_location) (.x _slam_attack_boundary_2_location)) (Math|Random|RandomFloatinRange (.y _slam_attack_boundary_1_location) (.y _slam_attack_boundary_2_location)) (.z _slam_attack_boundary_1_location)))
  (Game|SpawnActorfromClass "/Game/Blueprints/AI/Enemies/GolemBoss/Falling_Projectiles.Falling_Projectiles_C" (Math|Transform|MakeTransform (Variables|Default|GetSmall%20Projectile%20Location) "0, 0, 0" "1,1,1") "Undefined" 0 2.0 0)
  (Game|SpawnActorfromClass "/Game/Blueprints/AI/Enemies/GolemBoss/Attack_Indicator.Attack_Indicator_C" (Math|Transform|MakeTransform (Variables|Default|GetSmall%20Projectile%20Location) "0, 0, 0" "2.000000,2.000000,2.000000") "Undefined" 0 "1.000000,1.000000,1.000000" 2.0 true 0)
  (bind _counter (Utilities|FlowControl|DoN _returnvalue_4)
    (:Exit
      (Math|Integer|CompareInt _counter _returnvalue_4
        (:>
          (CallFunction|SmallSlamAttackReset :!label _label))
        (:==
          (goto _label))
        (:<
          (CallFunction|SmallSlamAttackFallingProjectiles))))))

(event Custom|Big%20Slam%20Attack%20Falling%20Projectiles
  (bind _phase (Variables|Default|GetPhase))
  (bind _slam_attack_boundary_1_location (Variables|Default|GetSlam%20Attack%20Boundary%201%20Location))
  (bind _slam_attack_boundary_2_location (Variables|Default|GetSlam%20Attack%20Boundary%202%20Location))
  (bind _returnvalue (* _phase 2))
  (bind _returnvalue_2 (- _returnvalue 3))
  (Utilities|FlowControl|Delay (Math|Random|RandomFloatinRange 0.5 2.0))
  (Variables|Default|SetLarge%20Projectile%20Location (Math|Vector|MakeVector (Math|Random|RandomFloatinRange (.x _slam_attack_boundary_1_location) (.x _slam_attack_boundary_2_location)) (Math|Random|RandomFloatinRange (.y _slam_attack_boundary_1_location) (.y _slam_attack_boundary_2_location)) (.z _slam_attack_boundary_1_location)))
  (Game|SpawnActorfromClass "/Game/Blueprints/AI/Enemies/GolemBoss/Large_Falling_Projectile.Large_Falling_Projectile_C" (Math|Transform|MakeTransform (Variables|Default|GetLarge%20Projectile%20Location) "0, 0, 0" "2.000000,2.000000,2.000000") "Undefined" 0 3.0 0)
  (Game|SpawnActorfromClass "/Game/Blueprints/AI/Enemies/GolemBoss/Attack_Indicator.Attack_Indicator_C" (Math|Transform|MakeTransform (Variables|Default|GetLarge%20Projectile%20Location) "0, 0, 0" "2.000000,2.000000,2.000000") "Undefined" 0 "1.500000,1.500000,1.500000" 3.0 true 0)
  (bind _counter (Utilities|FlowControl|DoN _returnvalue_2)
    (:Exit
      (Math|Integer|CompareInt _counter _returnvalue_2
        (:>
          (CallFunction|BigSlamProjectileReset :!label _label))
        (:==
          (goto _label))
        (:<
          (CallFunction|BigSlamAttackFallingProjectiles))))))

(event Custom|Small%20Slam%20Attack%20Reset
  (bind _phase (Variables|Default|GetPhase))
  (bind _returnvalue (Math|Conversions|ToFloat(Integer) _phase))
  (bind _returnvalue_2 (Math|Float|Power _returnvalue 1.5))
  (bind _returnvalue_3 (* 4 _returnvalue_2))
  (bind _returnvalue_4 (Math|Float|Ceil _returnvalue_3))
  (Utilities|FlowControl|DoN _returnvalue_4) ; enters at Reset
)

(event Custom|Big%20Slam%20Projectile%20Reset
  (bind _phase (Variables|Default|GetPhase))
  (bind _returnvalue (* _phase 2))
  (bind _returnvalue_2 (- _returnvalue 3))
  (Utilities|FlowControl|DoN _returnvalue_2) ; enters at Reset
)

(event Collision|EventHit
  (params (MyComp :type Primitive%20Component%20Object%20Reference) (Other :type Actor%20Object%20Reference) (OtherComp :type Primitive%20Component%20Object%20Reference) (bSelfMoved :type Boolean) (HitLocation :type Vector :default "0, 0, 0") (HitNormal :type Vector :default "0, 0, 0") (NormalImpulse :type Vector :default "0, 0, 0") (Hit :type Hit%20Result%20Structure%20%28by%20ref%29))
  (bind _asstun_bp (Utilities|Casting|CastToStunBP Other))
  (Actor|DestroyActor _asstun_bp)
  (Pawn|Components|CharacterMovement|DisableMovement (Variables|Character|GetCharacterMovement))
  (Utilities|FlowControl|Delay 3.0)
  (Pawn|Components|CharacterMovement|SetMovementMode (Variables|Character|GetCharacterMovement) "MOVE_Walking" 0))

(event EventBeginPlay
  (bind _returnvalue (Transformation|GetActorLocation))
  (Components|Activation|Deactivate (Variables|Character|GetCharacterMovement))
  (Variables|Default|SetSpawn%20Location _returnvalue)
  (Utilities|FlowControl|Delay 2.0)
  (Transformation|SetActorLocation (+ _returnvalue "0, 0,15000.000000") false false)
  (bind _asbp_default_game_mode (Utilities|Casting|CastToBP_Default_GameMode (Game|GetGameMode)))
  (Default|InitialEnemySpawns _asbp_default_game_mode "Gym" false)
  (Rendering|SetActorHiddenInGame false)
  (bind _returnvalue_2 (Game|SpawnActorfromClass "/Game/Blueprints/AI/Enemies/GolemBoss/SlamAttackSpline.SlamAttackSpline_C" (Math|Transform|MakeTransform "0, 0, 0" "0, 0, 0" "1,1,1") "Undefined" 0 0))
  (bind _output_get (Variables|Default|SetSpline%20Ref _returnvalue_2))
  (Spline|SetSplinePoints (Variables|/Game/Blueprints/AI/Enemies/GolemBoss/SlamAttackSpline.SlamAttackSpline_C|GetSpline _output_get) (Utilities|Array|MakeArray (Variables|Default|GetSpawn%20Location) (Transformation|GetActorLocation)) "World" true)
  (bind _spline_progress (Timeline|Initial%20Slam PlayFromStart)
    (:Update
      (Transformation|SetActorLocation (Spline|GetLocationatDistanceAlongSpline (Variables|/Game/Blueprints/AI/Enemies/GolemBoss/SlamAttackSpline.SlamAttackSpline_C|GetSpline (Variables|Default|GetSpline%20Ref)) (* (Spline|GetSplineLength (Variables|/Game/Blueprints/AI/Enemies/GolemBoss/SlamAttackSpline.SlamAttackSpline_C|GetSpline (Variables|Default|GetSpline%20Ref))) _spline_progress) "World") false false))
    (:Finished
      (CallFunction|DamageLoop)
      ;[1 1 1] Temporary Hack to make gym enemies spawn when boss is active, will fix later.
      (bind _asbp_default_game_mode_2 (Utilities|Casting|CastToBP_Default_GameMode (Game|GetGameMode)))
      (Variables|/Game/Blueprints/GameModes/BP_Default_GameMode.BP_Default_GameMode_C|SetEnemy%20List _asbp_default_game_mode_2 (Utilities|Array|MakeArray "/Game/Blueprints/AI/Enemies/Basketball/BP_Basketball.BP_Basketball_C" "/Game/Blueprints/AI/Enemies/AmericanFootball/BP_Football.BP_Football_C" "/Game/Blueprints/AI/Enemies/TennisBall/BP_Tennisball.BP_Tennisball_C"))
      (Variables|/Game/Blueprints/GameModes/BP_Default_GameMode.BP_Default_GameMode_C|SetBoss%20Active _asbp_default_game_mode_2 true)
      (Utilities|FlowControl|Delay 2.5)
      (CallFunction|InitialPhaseShift)
      (Components|Activation|Activate (Variables|Character|GetCharacterMovement) false)
      (AI|Components|Blackboard|SetValueasObject (AI|GetBlackboard 0) (Utilities|Name|MakeLiteralName "SelfActor") self)
      (bind _outactors (Actor|GetAllActorsOfClass "/Game/Blueprints/AI/Enemies/GolemBoss/Slam_Attack_Boundaries.Slam_Attack_Boundaries_C"))
      (for (_array_element _array_index) _outactors
        (if (== _array_index 0)
          (Variables|Default|SetSlam%20Attack%20Boundary%201%20Location (Transformation|GetActorLocation _array_element))
          (else
            (Variables|Default|SetSlam%20Attack%20Boundary%202%20Location (Transformation|GetActorLocation _array_element))))))
    (:Slam%20Animation%20Start
      (Components|Animation|PlayAnimation (Variables|Character|GetMesh) "/Game/Characters/Golum+Animations/Golum_LP_Anim_Gollum_Skeleton_0SlamAttackAnim2.Golum_LP_Anim_Gollum_Skeleton_0SlamAttackAnim2" false)
      (bind _returnvalue_3 (UserInterface|CreateWidget "/Game/UI_Folder/HUD/Boss_Health_Bar.Boss_Health_Bar_C"))
      (UserInterface|Viewport|AddtoViewport _returnvalue_3 0)
      (Variables|Default|SetHealth%20Bar%20Reference _returnvalue_3)
      (Variables|/Game/UI_Folder/HUD/Boss_Health_Bar.Boss_Health_Bar_C|SetBoss%20Reference _returnvalue_3 self)
      (bind _health_percent (Timeline|Health%20Bar%20Load PlayFromStart)
        (:Update
          (Variables|Default|SetHealth%20Percent _health_percent))))))

(event EventTick
  (params (DeltaSeconds :type Float%20%28single-precision%29)))

(event Game|Damage|EventAnyDamage
  (params (Damage :type Float%20%28single-precision%29) (DamageType :type Damage%20Type%20Object%20Reference) (InstigatedBy :type Controller%20Object%20Reference) (DamageCauser :type Actor%20Object%20Reference))
  (if (not (or (Variables|Default|GetPhase%20Shifting) (Variables|Default|GetInitial%20Invulnerability)))
    (bind _output_get (Variables|Default|SetHealth (Math|Float|Clamp(Float) (- (Variables|Default|GetHealth) Damage) (Utilities|Select :Index (Variables|Default|GetPhase) :Option%200 2.25e+03 :Option%201 1.5e+03 :Option%202 7.5e+02 :Option%203 0.0) 2.25e+03)))
    (Variables|Default|SetHealth%20Percent (/ (Variables|Default|GetHealth) (Variables|Default|GetMax%20Health)))
    (Math|Float|CompareFloat _output_get (Utilities|Select :Index (Variables|Default|GetPhase) :Option%200 2.25e+03 :Option%201 1.5e+03 :Option%202 7.5e+02 :Option%203 0.0)
      (:==
        _)
      (:<
        _))
    (if (<= (Variables|Default|GetHealth) 0.0)
      (Game|SpawnActorfromClass "/Game/Blueprints/AI/Enemies/GolemBoss/Boss_Death_Explosion.Boss_Death_Explosion_C" (Transformation|GetActorTransform) "Undefined" 0 0)
      (Actor|DestroyActor)
      (else
        (AI|Components|Blackboard|SetValueasBool (AI|GetBlackboard 0) (Utilities|Name|MakeLiteralName "Phase Switch") true)
        (Variables|Default|SetPhase%20Shifting true)))))

(fn ConstructionScript)