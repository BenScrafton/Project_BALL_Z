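; Ice cream enemy that chills the nearby player and is immobilized for seven seconds when hit by a StunBP.
; Tick moves a spawned ice decal with it, expanding or shrinking it through timelines by player distance, with hysteresis.
; Sphere3 overlap starts a sound and makes Tick progressively cut walk speed and double mouse smoothing.
; End overlap restores both, but sets Overlapping true when the player leaves, so the Tick effect resumes.
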(event OnComponentBeginOverlap(Sphere3)
  (params (OverlappedComponent :type Primitive%20Component%20Object%20Reference) (OtherActor :type Actor%20Object%20Reference) (OtherComp :type Primitive%20Component%20Object%20Reference) (OtherBodyIndex :type Integer) (bFromSweep :type Boolean) (SweepResult :type Hit%20Result%20Structure%20%28by%20ref%29))
  (bind _asbp_player (Utilities|Casting|CastToBP_Player OtherActor))
  (Variables|Default|Setplayer _asbp_player)
  (Variables|Default|Setoverlapping true)
  (Variables|Default|SetorigPlayerSpeed (Variables|/Script/Engine.CharacterMovementComponent|GetMaxWalkSpeed (Variables|/Script/Engine.Character|GetCharacterMovement (Variables|Default|Getplayer))))
  (Variables|Default|SetorigMouseSmoothing (Variables|/Game/Blueprints/Pawns/BP_Player.BP_Player_C|GetmouseSmoothingStrength (Variables|Default|Getplayer)))
  (bind _returnvalue (Audio|SpawnSound2D "/Game/Audio/Ice.Ice" 1.0 1.0 0.0 0))
  (Variables|Default|Set2dSound _returnvalue))

(event OnComponentEndOverlap(Sphere3)
  (params (OverlappedComponent :type Primitive%20Component%20Object%20Reference) (OtherActor :type Actor%20Object%20Reference) (OtherComp :type Primitive%20Component%20Object%20Reference) (OtherBodyIndex :type Integer))
  (Audio|Components|Audio|Stop (Variables|Default|Get2dSound))
  (Variables|Default|Setoverlapping (== OtherActor (Variables|Default|Getplayer)))
  (Variables|/Script/Engine.CharacterMovementComponent|SetMaxWalkSpeed (Variables|/Script/Engine.Character|GetCharacterMovement (Variables|Default|Getplayer)) (Variables|Default|GetorigPlayerSpeed))
  (Variables|/Game/Blueprints/Pawns/BP_Player.BP_Player_C|SetmouseSmoothingStrength (Variables|Default|Getplayer) (Variables|Default|GetorigMouseSmoothing)))

(event Custom|ShrinkDecal
  (Variables|Default|Setexpanded false)
  (bind _shrink (Timeline|ShrinkScale PlayFromStart)
    (:Update
      (Transformation|SetWorldScale3D (Variables|/Script/Engine.DecalActor|GetDecal (Variables|Default|GetDecal)) (Math|Vector|MakeVector 1.0 _shrink _shrink)))))

(event Custom|ExpandDecal
  (Variables|Default|Setexpanded true)
  (bind _expand (Timeline|ExpandScale PlayFromStart)
    (:Update
      (Transformation|SetWorldScale3D (Variables|/Script/Engine.DecalActor|GetDecal (Variables|Default|GetDecal)) (Math|Vector|MakeVector 1.0 _expand _expand)))))

(event Collision|EventHit
  (params (MyComp :type Primitive%20Component%20Object%20Reference) (Other :type Actor%20Object%20Reference) (OtherComp :type Primitive%20Component%20Object%20Reference) (bSelfMoved :type Boolean) (HitLocation :type Vector :default "0, 0, 0") (HitNormal :type Vector :default "0, 0, 0") (NormalImpulse :type Vector :default "0, 0, 0") (Hit :type Hit%20Result%20Structure%20%28by%20ref%29))
  (bind _asstun_bp (Utilities|Casting|CastToStunBP Other))
  (Actor|DestroyActor _asstun_bp)
  (Pawn|Components|CharacterMovement|DisableMovement (Variables|Character|GetCharacterMovement))
  (Utilities|FlowControl|Delay 7.0)
  (Pawn|Components|CharacterMovement|SetMovementMode (Variables|Character|GetCharacterMovement) "MOVE_Walking" 0))

(event Collision|EventActorBeginOverlap
  (params (OtherActor :type Actor%20Object%20Reference)))

(event EventTick
  (params (DeltaSeconds :type Float%20%28single-precision%29))
  (bind _player (Variables|Default|Getplayer))
  (bind _charactermovement (Variables|/Script/Engine.Character|GetCharacterMovement _player))
  (Transformation|SetActorLocation (Variables|Default|GetDecal) (Transformation|GetWorldLocation (Variables|Default|GetDecalSpawn)) false false)
  (CallFunction|HandleExpand)
  (CallFunction|HandleShrink)
  (if (Variables|Default|Getoverlapping)
    (if true
      (Variables|/Script/Engine.CharacterMovementComponent|SetMaxWalkSpeed _charactermovement (- (Variables|/Script/Engine.CharacterMovementComponent|GetMaxWalkSpeed _charactermovement) (* (Utilities|Time|GetWorldDeltaSeconds) 1e+02)))
      (Variables|/Game/Blueprints/Pawns/BP_Player.BP_Player_C|SetmouseSmoothingStrength (Variables|Default|Getplayer) (* (Variables|/Game/Blueprints/Pawns/BP_Player.BP_Player_C|GetmouseSmoothingStrength _player) 2.0)))))

(event EventBeginPlay
  (Audio|PlaySoundatLocation "/Game/Audio/Icecream_enemy__may_change_.Icecream_enemy__may_change_" "0, 0, 0" "0, 0, 0" 1.0 1.0 0.0 0 0 0)
  (bind _returnvalue (Game|SpawnActorfromClass "/Game/Blueprints/AI/Enemies/IceCream/Decal_Ice.Decal_Ice_C" (Math|Transform|MakeTransform (Transformation|GetWorldLocation (Variables|Default|GetDecalSpawn)) "0, 0, 0" "0.000000,0.000000,0.000000") "Undefined" 0 0))
  (Variables|Default|SetDecal _returnvalue))

(fn ConstructionScript)

(fn HandleExpand
  (if (and (< (Math|Vector|Distance(Vector) (Transformation|GetActorLocation) (Transformation|GetActorLocation (Game|Player|GetPlayerPawn 0))) 1e+03) (not (Variables|Default|Getexpanded)))
    (CallFunction|ExpandDecal)))

(fn HandleShrink
  (if (and (> (Math|Vector|Distance(Vector) (Transformation|GetActorLocation) (Transformation|GetActorLocation (Game|Player|GetPlayerPawn 0))) 1.1e+03) (Variables|Default|Getexpanded))
    (CallFunction|ShrinkDecal)))