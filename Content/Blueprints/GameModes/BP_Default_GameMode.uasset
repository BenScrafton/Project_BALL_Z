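; Default game mode that creates the main HUD and runs timed enemy waves with cooldowns until the room completes, plus a boss mid-phase countdown.
; A looping spawner picks random enemies by weight, throttled by live-enemy count and per-type limits.
; Box and line traces retry random points around the player until finding floor without walls, then roll elite types.
; Separate room-tagged initial spawns and an apparently unfinished wave-difficulty system are also included.
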(event Custom|Wave%20Cooldown
  (Utilities|FlowControl|Delay 1.0)
  (Math|Integer|DecrementInt (Variables|EnemySpawningVariables|GetWave%20Cooldown%20Timer)
    (:%20%20
      (Math|Integer|CompareInt (Variables|EnemySpawningVariables|GetWave%20Cooldown%20Timer)
        (:>
          (CallFunction|WaveCooldown))
        (:==
          (Math|Integer|IncrementInt (Variables|EnemySpawningVariables|GetWave%20Number) :!label _label
            (:%20%20
              (CallFunction|WaveStart))))
        (:<
          (goto _label))))))

(event Custom|Wave%20Start
  (bind _hud_reference (Variables|Default|GetHUD%20reference))
  (Variables|EnemySpawningVariables|SetWave%20Timer 30)
  (Variables|EnemySpawningVariables|SetWaveActive true)
  (Rendering|Components|TextRender|SetText (Variables|/Game/UI_Folder/HUD/MainHUD.MainHUD_C|GetWaveText _hud_reference) "")
  (Widget|SetVisibility (Variables|/Game/UI_Folder/HUD/MainHUD.MainHUD_C|GetWaveTimer _hud_reference) "Collapsed")
  (CallFunction|WaveCountdown))

(event Custom|Initial%20Enemy%20Spawns
  (params (Room :type Name))
  (bind _enemy_list (Variables|EnemySpawningVariables|GetEnemy%20List))
  ;[0.003922 0 0.2431] Initial Enemy Spawns
  (bind _outactors (Actor|GetAllActorsOfClasswithTag "/Game/Blueprints/AI/Enemies/Initial_Spawn_Locations.Initial_Spawn_Locations_C" Room))
  (Variables|Default|SetInitial%20Spawn%20Location _outactors)
  (Utilities|Array|Clear (Variables|EnemySpawningVariables|GetEnemies%20to%20Spawn))
  (for _index (range 0 4)
    (Utilities|Array|Add (Variables|EnemySpawningVariables|GetEnemies%20to%20Spawn) (Utilities|GetClassDisplayName (Utilities|Array|Get(acopy) _enemy_list (Math|Random|RandomIntegerinRange 0 (- (Utilities|Array|Length _enemy_list) 1))))))
  (for (_array_element _array_index) (Variables|EnemySpawningVariables|GetEnemies%20to%20Spawn)
    (bind _output_get (Variables|EnemySpawningVariables|SetEnemy%20To%20Spawn _array_element))
    (Math|Float|CompareFloat (.Value (Utilities|Map|Find (Variables|EnemySpawningVariables|GetEnemy%20Spawn%20Weights) _output_get)) 1.0
      (:>
        (Variables|EnemySpawningVariables|SetSpawn%20Weight (Math|Float|Truncate (- (.Value (Utilities|Map|Find (Variables|EnemySpawningVariables|GetEnemy%20Spawn%20Weights) _output_get)) 1.0)) :!label _label))
      (:==
        (goto _label))
      (:<
        (Variables|EnemySpawningVariables|SetSpawn%20Weight 0)))
    (for _index_2 (range 0 (Variables|EnemySpawningVariables|GetSpawn%20Weight))
      (CallFunction|EnemySpawn (Variables|EnemySpawningVariables|GetEnemy%20To%20Spawn) (+ (* "0,100.000000, 0" _index_2) (Transformation|GetActorLocation (Utilities|Array|Get(acopy) (Variables|Default|GetInitial%20Spawn%20Location) _array_index)))))))

(event Custom|Break%20Loop
  (bind _enemy_spawn_location (Variables|EnemySpawningVariables|GetEnemy%20Spawn%20Location))
  (bind _created_enemy (Variables|EnemySpawningVariables|GetCreated%20Enemy))
  ;[0.003922 0 0.2431] Enemy Spawn Loop
  ;;[0 1 0.9196] Box trace to check if there are walls or a floor in the spawn location
  (Utilities|Array|ForEachLoopwithBreak (stale Custom|Enemy%20Spawn%20Cycle _outhits)) ; enters at Break
)

(event Custom|Enemy%20Spawn%20Cycle
  (bind _returnvalue (Math|Random|RandomUnitVector))
  (bind _returnvalue_2 (Math|Random|RandomFloatinRange 1e+03 2.5e+03))
  (bind _returnvalue_3 (Game|GetPlayerCharacter 0))
  (bind _returnvalue_4 (Game|GetPlayerCharacter 0))
  (bind _array (Utilities|Array|MakeArray "ObjectTypeQuery1"))
  (bind _enemy_list (Variables|EnemySpawningVariables|GetEnemy%20List))
  (bind _created_enemy (Variables|EnemySpawningVariables|GetCreated%20Enemy))
  (bind _returnvalue_5 (* (Math|Vector|MakeVector (.x _returnvalue) (.y _returnvalue) 0.0) _returnvalue_2))
  (bind _returnvalue_6 (Transformation|GetActorLocation _returnvalue_4))
  (bind _array_2 (Utilities|Array|MakeArray _returnvalue_3))
  (bind _returnvalue_7 (+ _returnvalue_5 _returnvalue_6 "0,0,100.000000"))
  ;[0.003922 0 0.2431] Enemy Spawn Loop
  (Utilities|FlowControl|Delay 0.5)
  (Utilities|Array|Clear (Variables|EnemySpawningVariables|GetEnemies%20to%20Spawn))
  (if (Variables|EnemySpawningVariables|GetBoss%20Active)
    ;;[0 1 0.9196] Check if there's too many enemies in the game
    (bind _outactors (Actor|GetAllActorsOfClass "/Game/Blueprints/AI/Enemies/BP_AIEnemyController.BP_AIEnemyController_C" :!label _label))
    (Math|Integer|CompareInt (Utilities|Array|Length _outactors) 10
      (:>
        (Utilities|FlowControl|Delay 1.0 :!label _label_2)
        (CallFunction|EnemySpawnCycle))
      (:==
        (Utilities|FlowControl|Delay (Math|Random|RandomFloatinRange 4.0 7.0) :!label _label_3)
        (if (Variables|EnemySpawningVariables|GetBoss%20Active)
          (goto _label_2)
          (else
            (for _index (range 0 1)
              (Utilities|Array|Add (Variables|EnemySpawningVariables|GetEnemies%20to%20Spawn) (Utilities|GetClassDisplayName (Utilities|Array|Get(acopy) _enemy_list (Math|Random|RandomIntegerinRange 0 (- (Utilities|Array|Length _enemy_list) 1))))))
            ;;[0 1 0.9196] Chance based on the number of enemies that are currently alive to continue with the spawn loop, down to a minimum of about 23% when there are 9 enemies in play.
            (bind _outactors_2 (Actor|GetAllActorsOfClass "/Game/Blueprints/AI/BP_EnemyAIController.BP_EnemyAIController_C"))
            (if (Math|Random|RandomBoolwithWeight (Math|Float|Power 0.85 (Math|Conversions|ToFloat(Integer) (Utilities|Array|Length _outactors_2))))
              (for _array_element (Variables|EnemySpawningVariables|GetEnemies%20to%20Spawn)
                (bind _output_get (Variables|EnemySpawningVariables|SetEnemy%20To%20Spawn _array_element))
                (Math|Float|CompareFloat (.Value (Utilities|Map|Find (Variables|EnemySpawningVariables|GetEnemy%20Spawn%20Weights) _output_get)) 1.0
                  (:>
                    (Variables|EnemySpawningVariables|SetSpawn%20Weight (Math|Float|Truncate (- (.Value (Utilities|Map|Find (Variables|EnemySpawningVariables|GetEnemy%20Spawn%20Weights) _output_get)) 1.0)) :!label _label_4)
                    (for _index_2 (range 0 (Variables|EnemySpawningVariables|GetSpawn%20Weight)) :!label _label_5
                      (bind _returnvalue_8 (CallFunction|EnemySpawnLimits))
                      (if _returnvalue_8
                        (Variables|EnemySpawningVariables|SetEnemy%20Spawn%20Location _returnvalue_7)
                        ;;[0 1 0.9196] Box trace to check if there are walls or a floor in the spawn location
                        (bind _outhits (Class|KismetSystemLibrary|BoxTraceMultiforObjects _returnvalue_7 (- _returnvalue_7 "0, 0,500.000000") "200.000000,200.000000,200.000000" "0, 0, 0" _array false _array_2 "None" true))
                        (bind _array_element_2 (Utilities|Array|ForEachLoopwithBreak _outhits)
                          (:LoopBody
                            (Utilities|IsValid (.HitActor (Collision|BreakHitResult _array_element_2))
                              (:Is%20Valid
                                (if (Actor|ActorHasTag (.HitActor (Collision|BreakHitResult _array_element_2)) "Wall")
                                  (Variables|EnemySpawningVariables|SetHit%20Wall true)
                                  (CallFunction|BreakLoop)))))
                          (:Completed
                            (bind _outhits_2 (Class|KismetSystemLibrary|LineTraceMultiforObjects (Variables|EnemySpawningVariables|GetEnemy%20Spawn%20Location) (- (Variables|EnemySpawningVariables|GetEnemy%20Spawn%20Location) "0, 0,500.000000") _array false _array_2 "None" true))
                            (bind _array_element_3 (Utilities|Array|ForEachLoopwithBreak _outhits_2)
                              (:LoopBody
                                (Utilities|IsValid (.HitActor (Collision|BreakHitResult _array_element_3))
                                  (:Is%20Valid
                                    (if (Actor|ActorHasTag (.HitActor (Collision|BreakHitResult _array_element_3)) "Floor")
                                      (Variables|EnemySpawningVariables|SetHit%20Floor true)
                                      (CallFunction|BreakFloorLoop)))))
                              (:Completed
                                (if (Variables|EnemySpawningVariables|GetHit%20Floor)
                                  (if (Variables|EnemySpawningVariables|GetHit%20Wall)
                                    (Variables|EnemySpawningVariables|SetHit%20Wall false :!label _label_6)
                                    (Variables|EnemySpawningVariables|SetHit%20Floor false)
                                    (CallFunction|RetryTrace)
                                    (else
                                      (Variables|EnemySpawningVariables|SetHit%20Wall false)
                                      (Variables|EnemySpawningVariables|SetHit%20Floor false)
                                      (if (Math|Random|RandomBoolwithWeight 0.975)
                                        (Variables|EnemySpawningVariables|SetElite%20Type%20Chosen "NewEnumerator5")
                                        (else
                                          (Variables|EnemySpawningVariables|SetElite%20Type%20Chosen (Utilities|Select :Index (Math|Random|RandomIntegerinRange 0 1) :Option%200 "NewEnumerator0" :Option%201 "NewEnumerator1" :Option%202 "NewEnumerator2" :Option%203 "NewEnumerator3" :Option%204 "NewEnumerator4" :Option%205 "NewEnumerator6"))))
                                      (CallFunction|EnemySpawn (Variables|EnemySpawningVariables|GetEnemy%20To%20Spawn) (Variables|EnemySpawningVariables|GetEnemy%20Spawn%20Location))
                                      (Utilities|IsValid _created_enemy
                                        (:Is%20Valid
                                          (bind _asbp_aienemy_controller (Utilities|Casting|CastToBP_AIEnemyController (AI|GetAIController _created_enemy)))
                                          (Variables|/Game/Blueprints/AI/Enemies/BP_AIEnemyController.BP_AIEnemyController_C|SetElite%20Type _asbp_aienemy_controller (Variables|EnemySpawningVariables|GetElite%20Type%20Chosen))))))
                                  (else
                                    (goto _label_6))))))))))
                  (:==
                    (goto _label_4))
                  (:<
                    (if (Math|Random|RandomBoolwithWeight (.Value (Utilities|Map|Find (Variables|EnemySpawningVariables|GetEnemy%20Spawn%20Weights) _output_get)))
                      (Variables|EnemySpawningVariables|SetSpawn%20Weight 0)
                      (goto _label_5))))))
            (CallFunction|EnemySpawnCycle))))
      (:<
        (goto _label_3)))
    (elif (not (Variables|EnemySpawningVariables|GetWaveActive))
      (goto _label_2)
      (else
        (goto _label)))))

(event Custom|Retry%20Elite
  (bind _created_enemy (Variables|EnemySpawningVariables|GetCreated%20Enemy))
  ;[0.003922 0 0.2431] Enemy Spawn Loop
  (Utilities|FlowControl|Delay 0.05)
  (if (Math|Random|RandomBoolwithWeight 0.975)
    (Variables|EnemySpawningVariables|SetElite%20Type%20Chosen "NewEnumerator5")
    (else
      (Variables|EnemySpawningVariables|SetElite%20Type%20Chosen (Utilities|Select :Index (Math|Random|RandomIntegerinRange 0 1) :Option%200 "NewEnumerator0" :Option%201 "NewEnumerator1" :Option%202 "NewEnumerator2" :Option%203 "NewEnumerator3" :Option%204 "NewEnumerator4" :Option%205 "NewEnumerator6"))))
  (CallFunction|EnemySpawn (Variables|EnemySpawningVariables|GetEnemy%20To%20Spawn) (Variables|EnemySpawningVariables|GetEnemy%20Spawn%20Location))
  (Utilities|IsValid _created_enemy
    (:Is%20Valid
      (bind _asbp_aienemy_controller (Utilities|Casting|CastToBP_AIEnemyController (AI|GetAIController _created_enemy)))
      (Variables|/Game/Blueprints/AI/Enemies/BP_AIEnemyController.BP_AIEnemyController_C|SetElite%20Type _asbp_aienemy_controller (Variables|EnemySpawningVariables|GetElite%20Type%20Chosen)))))

(event Custom|Break%20Floor%20Loop
  (bind _created_enemy (Variables|EnemySpawningVariables|GetCreated%20Enemy))
  ;[0.003922 0 0.2431] Enemy Spawn Loop
  (Utilities|Array|ForEachLoopwithBreak (stale Custom|Enemy%20Spawn%20Cycle _outhits_2)) ; enters at Break
)

(event Custom|Retry%20Trace
  (bind _returnvalue (Math|Random|RandomUnitVector))
  (bind _returnvalue_2 (Math|Random|RandomFloatinRange 1e+03 2.5e+03))
  (bind _returnvalue_3 (Game|GetPlayerCharacter 0))
  (bind _returnvalue_4 (Game|GetPlayerCharacter 0))
  (bind _array (Utilities|Array|MakeArray "ObjectTypeQuery1"))
  (bind _created_enemy (Variables|EnemySpawningVariables|GetCreated%20Enemy))
  (bind _returnvalue_5 (* (Math|Vector|MakeVector (.x _returnvalue) (.y _returnvalue) 0.0) _returnvalue_2))
  (bind _returnvalue_6 (Transformation|GetActorLocation _returnvalue_4))
  (bind _array_2 (Utilities|Array|MakeArray _returnvalue_3))
  (bind _returnvalue_7 (+ _returnvalue_5 _returnvalue_6 "0,0,100.000000"))
  ;[0.003922 0 0.2431] Enemy Spawn Loop
  (Utilities|FlowControl|Delay 0.075)
  (Variables|EnemySpawningVariables|SetEnemy%20Spawn%20Location _returnvalue_7)
  ;;[0 1 0.9196] Box trace to check if there are walls or a floor in the spawn location
  (bind _outhits (Class|KismetSystemLibrary|BoxTraceMultiforObjects _returnvalue_7 (- _returnvalue_7 "0, 0,500.000000") "200.000000,200.000000,200.000000" "0, 0, 0" _array false _array_2 "None" true))
  (bind _array_element (Utilities|Array|ForEachLoopwithBreak _outhits)
    (:LoopBody
      (Utilities|IsValid (.HitActor (Collision|BreakHitResult _array_element))
        (:Is%20Valid
          (if (Actor|ActorHasTag (.HitActor (Collision|BreakHitResult _array_element)) "Wall")
            (Variables|EnemySpawningVariables|SetHit%20Wall true)
            (CallFunction|BreakLoop)))))
    (:Completed
      (bind _outhits_2 (Class|KismetSystemLibrary|LineTraceMultiforObjects (Variables|EnemySpawningVariables|GetEnemy%20Spawn%20Location) (- (Variables|EnemySpawningVariables|GetEnemy%20Spawn%20Location) "0, 0,500.000000") _array false _array_2 "None" true))
      (bind _array_element_2 (Utilities|Array|ForEachLoopwithBreak _outhits_2)
        (:LoopBody
          (Utilities|IsValid (.HitActor (Collision|BreakHitResult _array_element_2))
            (:Is%20Valid
              (if (Actor|ActorHasTag (.HitActor (Collision|BreakHitResult _array_element_2)) "Floor")
                (Variables|EnemySpawningVariables|SetHit%20Floor true)
                (CallFunction|BreakFloorLoop)))))
        (:Completed
          (if (Variables|EnemySpawningVariables|GetHit%20Floor)
            (if (Variables|EnemySpawningVariables|GetHit%20Wall)
              (Variables|EnemySpawningVariables|SetHit%20Wall false :!label _label)
              (Variables|EnemySpawningVariables|SetHit%20Floor false)
              (CallFunction|RetryTrace)
              (else
                (Variables|EnemySpawningVariables|SetHit%20Wall false)
                (Variables|EnemySpawningVariables|SetHit%20Floor false)
                (if (Math|Random|RandomBoolwithWeight 0.975)
                  (Variables|EnemySpawningVariables|SetElite%20Type%20Chosen "NewEnumerator5")
                  (else
                    (Variables|EnemySpawningVariables|SetElite%20Type%20Chosen (Utilities|Select :Index (Math|Random|RandomIntegerinRange 0 1) :Option%200 "NewEnumerator0" :Option%201 "NewEnumerator1" :Option%202 "NewEnumerator2" :Option%203 "NewEnumerator3" :Option%204 "NewEnumerator4" :Option%205 "NewEnumerator6"))))
                (CallFunction|EnemySpawn (Variables|EnemySpawningVariables|GetEnemy%20To%20Spawn) (Variables|EnemySpawningVariables|GetEnemy%20Spawn%20Location))
                (Utilities|IsValid _created_enemy
                  (:Is%20Valid
                    (bind _asbp_aienemy_controller (Utilities|Casting|CastToBP_AIEnemyController (AI|GetAIController _created_enemy)))
                    (Variables|/Game/Blueprints/AI/Enemies/BP_AIEnemyController.BP_AIEnemyController_C|SetElite%20Type _asbp_aienemy_controller (Variables|EnemySpawningVariables|GetElite%20Type%20Chosen))))))
            (else
              (goto _label))))))))

(event Custom|Boss%20Mid-Phase%20Wave%20Start
  (params (Boss%20Reference :type BP%20Golem%20Boss%20Object%20Reference))
  (Variables|Default|SetBoss%20Reference Boss%20Reference)
  (Variables|EnemySpawningVariables|SetWave%20Timer 60)
  (Variables|EnemySpawningVariables|SetBoss%20Active false)
  (Widget|SetVisibility (Variables|/Game/UI_Folder/HUD/MainHUD.MainHUD_C|GetWaveTimer (Variables|Default|GetHUD%20reference)) "Collapsed")
  (CallFunction|BossMid-PhaseWaveCountdown))

(event Custom|Boss%20Mid-Phase%20Wave%20Countdown
  (Utilities|FlowControl|Delay 0.1)
  (Math|Integer|DecrementInt (Variables|EnemySpawningVariables|GetWave%20Timer)
    (:%20%20
      (Math|Integer|CompareInt (Variables|EnemySpawningVariables|GetWave%20Timer)
        (:>
          (CallFunction|BossMid-PhaseWaveCountdown))
        (:==
          (Variables|EnemySpawningVariables|SetBoss%20Active true :!label _label))
        (:<
          (goto _label))))))

(event Custom|Wave%20Countdown
  (bind _hud_reference (Variables|Default|GetHUD%20reference))
  (bind _hud_reference_2 (Variables|Default|GetHUD%20reference))
  (Utilities|FlowControl|Delay 1.0)
  (Math|Integer|DecrementInt (Variables|EnemySpawningVariables|GetWave%20Timer)
    (:%20%20
      (Math|Integer|CompareInt (Variables|EnemySpawningVariables|GetWave%20Timer)
        (:>
          (CallFunction|WaveCountdown))
        (:==
          (Math|Integer|CompareInt (Variables|EnemySpawningVariables|GetWave%20Number) 3 :!label _label
            (:>
              (Rendering|Components|TextRender|SetText (Variables|/Game/UI_Folder/HUD/MainHUD.MainHUD_C|GetWaveText _hud_reference) "Room Complete! Proceed To The Next Room To Continue" :!label _label_2)
              (Widget|SetVisibility (Variables|/Game/UI_Folder/HUD/MainHUD.MainHUD_C|GetWaveTimer _hud_reference) "Collapsed")
              (Widget|SetVisibility (Variables|/Game/UI_Folder/HUD/MainHUD.MainHUD_C|GetWaveText (Variables|Default|GetHUD%20reference)) "Visible")
              (Variables|EnemySpawningVariables|SetWaveActive false)
              (Variables|Default|SetWaves%20Completed true))
            (:==
              (goto _label_2))
            (:<
              (Rendering|Components|TextRender|SetText (Variables|/Game/UI_Folder/HUD/MainHUD.MainHUD_C|GetWaveText _hud_reference_2) "Wave Complete!")
              (Widget|SetVisibility (Variables|/Game/UI_Folder/HUD/MainHUD.MainHUD_C|GetWaveTimer _hud_reference_2) "Collapsed")
              (Widget|SetVisibility (Variables|/Game/UI_Folder/HUD/MainHUD.MainHUD_C|GetWaveText (Variables|Default|GetHUD%20reference)) "Visible")
              (Utilities|FlowControl|Delay 2.0)
              (Variables|EnemySpawningVariables|SetWave%20Cooldown%20Timer 15)
              (Rendering|Components|TextRender|SetText (Variables|/Game/UI_Folder/HUD/MainHUD.MainHUD_C|GetWaveText (Variables|Default|GetHUD%20reference)) "Prepare For The Next Wave")
              (Variables|EnemySpawningVariables|SetWaveActive false)
              (Widget|SetVisibility (Variables|/Game/UI_Folder/HUD/MainHUD.MainHUD_C|GetWaveTimer (Variables|Default|GetHUD%20reference)) "Visible")
              (CallFunction|WaveCooldown))))
        (:<
          (goto _label))))))

(event EventBeginPlay
  (bind _asbp_player (Utilities|Casting|CastToBP_Player (Game|GetPlayerCharacter 0)))
  (Variables|/Game/Blueprints/Pawns/BP_Player.BP_Player_C|SetIs%20Invincible _asbp_player false)
  (Variables|EnemySpawningVariables|SetSpawn%20Credits 50)
  (bind _returnvalue (UserInterface|CreateWidget "/Game/UI_Folder/HUD/MainHUD.MainHUD_C"))
  (Variables|Default|SetHUD%20reference _returnvalue)
  (UserInterface|Viewport|AddtoViewport _returnvalue 0)
  (Variables|/Game/UI_Folder/HUD/MainHUD.MainHUD_C|SetGamemode%20Reference (Variables|Default|GetHUD%20reference) self)
  (bind _asbp_player_2 (Utilities|Casting|CastToBP_Player (Game|Player|GetPlayerPawn 0)))
  (Variables|/Game/Blueprints/Pawns/BP_Player.BP_Player_C|SetHUD%20Reference _asbp_player_2 (Variables|Default|GetHUD%20reference))
  (Utilities|FlowControl|Delay 2.0)
  (CallFunction|WaveStart)
  (CallFunction|EnemySpawnCycle))

(event EventTick
  (params (DeltaSeconds :type Float%20%28single-precision%29)))

(fn ConstructionScript)

(fn NewWaveSetup
  (Math|Integer|IncrementInt (Variables|Default|GetcurrentWave)
    (:%20%20
      (CallFunction|IncreaseWaveDifficulty)
      (Utilities|Time|SetTimerbyFunctionName 0 "SpawnWave" (Variables|Default|GetEnemySpawnFrequency) true))))

(fn SpawnEnemy
  (bind _spawnpoint (CallFunction|ChooseRandomSpawnPoint))
  (Utilities|IsValid _spawnpoint))

(fn ChooseRandomSpawnPoint
  (bind _outactors (Actor|GetAllActorsOfClass "/Script/Engine.TargetPoint"))
  (return (Utilities|Array|Get(acopy) _outactors (Math|Random|RandomIntegerinRange 0 (Utilities|Array|LastIndex _outactors)))))

(fn RegisterEnemyDeath
  (params (enemy :type BP%20Enemy%20Object%20Reference%20%28by%20ref%29))
  (Utilities|Array|RemoveItem (Variables|Default|Getenemies) enemy)
  (if (CallFunction|IsWaveOver)
    _))

(fn IsWaveOver
  (return (and (== (Variables|Default|GetenemySpawnsRemaining) 0) (== (Utilities|Array|Length (Variables|Default|Getenemies)) 0))))

(fn IncreaseWaveDifficulty
  (bind _output_get (Variables|Default|SetwaveDifficulty (Math|Float|Round (* (Variables|Default|GetwaveDifficulty) (Variables|Default|GetdifficultyMultiplier)))))
  (Variables|Default|SetenemySpawnsRemaining _output_get)
  (Variables|Default|SetEnemySpawnFrequency (/ (Variables|Default|GetEnemySpawnFrequency) (Variables|Default|GetdifficultyMultiplier))))

(fn EnemySpawn
  (params (Enemy%20To%20Spawn :type String) (Spawn%20Location :type Vector))
  ;[0.003922 0 0.2431] Every time an enemy is added to the game, add them to the empty slots here
  (switch string Enemy%20To%20Spawn
    (:BP_Basketball_C
      (bind _returnvalue (AI|SpawnAIFromClass "/Game/Blueprints/AI/Enemies/Basketball/BP_Basketball.BP_Basketball_C" "/Game/Blueprints/AI/Enemies/Basketball/BT_Basketball.BT_Basketball" Spawn%20Location "0, 0, 0" false 0))
      (Variables|EnemySpawningVariables|SetCreated%20Enemy _returnvalue))
    (:BP_Football_C
      (bind _returnvalue_2 (AI|SpawnAIFromClass "/Game/Blueprints/AI/Enemies/AmericanFootball/BP_Football.BP_Football_C" "/Game/Blueprints/AI/Enemies/AmericanFootball/BT_Football.BT_Football" Spawn%20Location "0, 0, 0" false 0))
      (Variables|EnemySpawningVariables|SetCreated%20Enemy _returnvalue_2))
    (:BP_Tennisball_C
      (bind _returnvalue_3 (AI|SpawnAIFromClass "/Game/Blueprints/AI/Enemies/TennisBall/BP_Tennisball.BP_Tennisball_C" "/Game/Blueprints/AI/Enemies/TennisBall/BT_TennisBall.BT_Tennisball" Spawn%20Location "0, 0, 0" false 0))
      (Variables|EnemySpawningVariables|SetCreated%20Enemy _returnvalue_3))
    (:BP_PaintBrush_C
      (bind _returnvalue_4 (AI|SpawnAIFromClass "/Game/Blueprints/AI/Enemies/PaintBrush/BP_PaintBrush.BP_PaintBrush_C" 0 Spawn%20Location "0, 0, 0" false 0))
      (Variables|EnemySpawningVariables|SetCreated%20Enemy _returnvalue_4))
    (:BP_PaintPot_C
      (bind _returnvalue_5 (AI|SpawnAIFromClass "/Game/Blueprints/AI/Enemies/PaintPot/BP_PaintPot.BP_PaintPot_C" 0 Spawn%20Location "0, 0, 0" false 0))
      (Variables|EnemySpawningVariables|SetCreated%20Enemy _returnvalue_5))
    (:BP_PaintRoller_C
      (bind _returnvalue_6 (AI|SpawnAIFromClass "/Game/Blueprints/AI/Enemies/PaintRoller/BP_PaintRoller.BP_PaintRoller_C" 0 Spawn%20Location "0, 0, 0" false 0))
      (Variables|EnemySpawningVariables|SetCreated%20Enemy _returnvalue_6))
    (:BP_Fruit_C
      (bind _returnvalue_7 (AI|SpawnAIFromClass "/Game/Blueprints/AI/Enemies/Fruit/BP_Fruit.BP_Fruit_C" 0 Spawn%20Location "0, 0, 0" false 0))
      (Variables|EnemySpawningVariables|SetCreated%20Enemy _returnvalue_7))
    (:BP_Burger_C
      (bind _returnvalue_8 (AI|SpawnAIFromClass "/Game/Blueprints/AI/Enemies/Burger/BP_Burger.BP_Burger_C" 0 Spawn%20Location "0, 0, 0" false 0))
      (Variables|EnemySpawningVariables|SetCreated%20Enemy _returnvalue_8))
    (:BP_IceCream_C
      (bind _returnvalue_9 (AI|SpawnAIFromClass "/Game/Blueprints/AI/Enemies/IceCream/BP_IceCream.BP_IceCream_C" 0 Spawn%20Location "0, 0, 0" false 0))
      (Variables|EnemySpawningVariables|SetCreated%20Enemy _returnvalue_9)))
  (Utilities|Casting|CastToBP_AIEnemyController (AI|GetAIController (Variables|EnemySpawningVariables|GetCreated%20Enemy)))
  (return (Variables|EnemySpawningVariables|GetCreated%20Enemy)))

(fn EnemySpawnLimits
  (switch string (Variables|EnemySpawningVariables|GetEnemy%20To%20Spawn)
    (:BP_Basketball_C
      (bind _outactors (Actor|GetAllActorsOfClass "/Game/Blueprints/AI/Enemies/Basketball/BP_AIBasketballController.BP_AIBasketballController_C"))
      (LocalVariables|SetBelow%20Limit (< (Utilities|Array|Length _outactors) 3))
      (return (LocalVariables|GetBelow%20Limit)))
    (:BP_Football_C
      (bind _outactors_2 (Actor|GetAllActorsOfClass "/Game/Blueprints/AI/Enemies/AmericanFootball/BP_AIFootballController.BP_AIFootballController_C"))
      (LocalVariables|SetBelow%20Limit (< (Utilities|Array|Length _outactors_2) 3))
      (return (LocalVariables|GetBelow%20Limit)))
    (:BP_Tennisball_C
      (LocalVariables|SetBelow%20Limit true)
      (return (LocalVariables|GetBelow%20Limit)))
    (:BP_PaintBrush_C
      (LocalVariables|SetBelow%20Limit true)
      (return (LocalVariables|GetBelow%20Limit)))
    (:BP_PaintPot_C
      (bind _outactors_3 (Actor|GetAllActorsOfClass "/Game/Blueprints/AI/Enemies/PaintPot/BP_AIPaintPot.BP_AIPaintPot_C"))
      (LocalVariables|SetBelow%20Limit (< (Utilities|Array|Length _outactors_3) 3))
      (return (LocalVariables|GetBelow%20Limit)))
    (:BP_PaintRoller_C
      (bind _outactors_4 (Actor|GetAllActorsOfClass "/Game/Blueprints/AI/Enemies/PaintRoller/BP_PaintRoller.BP_PaintRoller_C"))
      (LocalVariables|SetBelow%20Limit (< (Utilities|Array|Length _outactors_4) 3)))
    (:BP_Fruit_C
      (LocalVariables|SetBelow%20Limit true)
      (return (LocalVariables|GetBelow%20Limit)))
    (:BP_Burger_C
      (bind _outactors_5 (Actor|GetAllActorsOfClass "/Game/Blueprints/AI/Enemies/Burger/BP_Burger.BP_Burger_C"))
      (LocalVariables|SetBelow%20Limit (< (Utilities|Array|Length _outactors_5) 5))
      (return (LocalVariables|GetBelow%20Limit)))
    (:BP_IceCream_C
      (bind _outactors_6 (Actor|GetAllActorsOfClass "/Game/Blueprints/AI/Enemies/IceCream/BP_IceCream.BP_IceCream_C"))
      (LocalVariables|SetBelow%20Limit (< (Utilities|Array|Length _outactors_6) 1))
      (return (LocalVariables|GetBelow%20Limit)))))