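; StunBP is a pickup actor that adds one to the player's StunCount when the player interacts with it.
; It enables input from player controller 0 on BeginPlay so it can receive the Interact action itself.
; Overlap events on InteractSphere cache the BP_Player and open or close a gate, so Interact only works while the player is in range.
; A successful interact increments the count and destroys the actor.
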(event OnComponentBeginOverlap(InteractSphere)
  (params (OverlappedComponent :type Primitive%20Component%20Object%20Reference) (OtherActor :type Actor%20Object%20Reference) (OtherComp :type Primitive%20Component%20Object%20Reference) (OtherBodyIndex :type Integer) (bFromSweep :type Boolean) (SweepResult :type Hit%20Result%20Structure%20%28by%20ref%29))
  (bind _asbp_player (Utilities|Casting|CastToBP_Player OtherActor))
  (Utilities|FlowControl|Gate true) ; enters at Open
)

(event OnComponentEndOverlap(InteractSphere)
  (params (OverlappedComponent :type Primitive%20Component%20Object%20Reference) (OtherActor :type Actor%20Object%20Reference) (OtherComp :type Primitive%20Component%20Object%20Reference) (OtherBodyIndex :type Integer))
  (Utilities|Casting|CastToBP_Player OtherActor)
  (Utilities|FlowControl|Gate true) ; enters at Close
)

(event EventBeginPlay
  (Input|EnableInput (Game|GetPlayerController 0)))

(event Input|ActionEvents|InputActionInteract
  (params (Key :type Key%20Structure :default "None"))
  (:Pressed
    (Utilities|FlowControl|Gate true
      (:Exit
        (bind _result (Math|Integer|IncrementInt (Variables|/Game/Blueprints/Pawns/BP_Player.BP_Player_C|GetStunCount (stale OnComponentBeginOverlap(InteractSphere) _asbp_player)))
          (:%20%20
            (Variables|/Game/Blueprints/Pawns/BP_Player.BP_Player_C|SetStunCount (stale OnComponentBeginOverlap(InteractSphere) _asbp_player) _result)
            (Actor|DestroyActor)))))))

(fn ConstructionScript)