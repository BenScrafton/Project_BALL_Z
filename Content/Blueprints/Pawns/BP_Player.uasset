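; Player character for a top-down action game, with movement, mouse or gamepad aim, dodge, stun throws, pausing and heart-based health.
; Tick times attack holds for light attacks via the socketed weapon or heavy attacks on nearby enemies, and updates aim and dodge movement.
; Damage removes hearts, then triggers flashing invincibility or death UI.
; A looping box trace fades MeshPlacer objects blocking the camera.
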(event Custom|Camera%20Collision%20Loop
  (CallFunction|CameraCollisionFunction)
  (Utilities|FlowControl|Delay 0.2)
  (CallFunction|CameraCollisionLoop))

(event Custom|KnockDown
  (Variables|Default|SetisKnockedDown true)
  (Variables|PlayerMovement|SetcanDash/Dodge true)
  (Animation|Montage|PlayMontage (Variables|Character|GetMesh) "/Game/ArtAssets/Temp/KidCharacter/Animations/PlayerKnockedDown.PlayerKnockedDown" 2.0
    (:OnBlendOut
      (Animation|Montage|PlayMontage (Variables|Character|GetMesh) "/Game/ArtAssets/Temp/KidCharacter/Animations/PlayerGetUp.PlayerGetUp" 2.0
        (:OnBlendOut
          (Variables|Default|SetisKnockedDown false))))))

(event Custom|Visibility%20Change%20Reset
  ;[1 1 1] Temporary Invincibility Flash, Can Be Changed Later
  (Utilities|FlowControl|DoN 60) ; enters at Reset
)

(event Custom|Visibility%20Change%20Repeat
  ;[1 1 1] Temporary Invincibility Flash, Can Be Changed Later
  (bind _counter (Utilities|FlowControl|DoN 60)
    (:Exit
      (Utilities|FlowControl|FlipFlop
        (:A
          (Rendering|SetVisibility (Variables|Character|GetMesh) false false)
          (Utilities|FlowControl|Delay 0.1))
        (:B
          (Rendering|SetVisibility (Variables|Character|GetMesh) true false)
          (Utilities|FlowControl|Delay 0.1)))
      (Math|Integer|CompareInt _counter 25
        (:>
          (CallFunction|VisibilityChangeReset :!label _label)
          (Variables|Default|SetIs%20Invincible false)
          (Rendering|SetVisibility (Variables|Character|GetMesh) true false))
        (:==
          (goto _label))
        (:<
          (CallFunction|VisibilityChangeRepeat))))))

(event Custom|Update%20Hearts
  (for _index (range 0 2)
    (if (< _index (Variables|Default|Gethearts))
      (Class|Image|SetBrush (Utilities|Array|Get(acopy) (Variables|/Game/UI_Folder/HUD/MainHUD.MainHUD_C|GetHeart%20References (Variables|Default|GetHUD%20Reference)) _index) (Utilities|Struct|MakeSlateBrush "(X=56.000000,Y=47.000000)" "(Left=0.000000,Top=0.000000,Right=0.000000,Bottom=0.000000)" "(SpecifiedColor=(R=1.000000,G=1.000000,B=1.000000,A=1.000000),ColorUseRule=UseColor_Specified)" "/Game/UI_Folder/UI_Assets/Full_Heart_Larger1.Full_Heart_Larger1" "Image" "NoTile" "NoMirror"))
      (else
        (Class|Image|SetBrush (Utilities|Array|Get(acopy) (Variables|/Game/UI_Folder/HUD/MainHUD.MainHUD_C|GetHeart%20References (Variables|Default|GetHUD%20Reference)) _index) (Utilities|Struct|MakeSlateBrush "(X=56.000000,Y=47.000000)" "(Left=0.000000,Top=0.000000,Right=0.000000,Bottom=0.000000)" "(SpecifiedColor=(R=1.000000,G=1.000000,B=1.000000,A=1.000000),ColorUseRule=UseColor_Specified)" "/Game/UI_Folder/UI_Assets/Empty_Heart_Larger1.Empty_Heart_Larger1" "Image" "NoTile" "NoMirror"))))))

(event EventBeginPlay
  (bind _returnvalue (Game|GetPlayerController 0))
  (Variables|/Script/Engine.PlayerController|SetbShowMouseCursor _returnvalue true)
  (Class|PlayerController|SetMouseCursorWidget _returnvalue "Crosshairs")
  (CallFunction|CameraCollisionLoop)
  (CallFunction|EquipWeapon "/Game/A0051431-CF-Folder/Weapons/Broom/ChildBroomBP/BP_BroomStarterWeapon.BP_BroomStarterWeapon_C")
  (Variables|Default|SetWeaponAttached%20? false))

(event EventTick
  (params (DeltaSeconds :type Float%20%28single-precision%29))
  (if (CallFunction|GetIsAlive)
    (Combat|ProcessCombat)
    (CharacterMovement|ProcessPlayerMovement)))

(event Game|Damage|EventAnyDamage
  (params (Damage :type Float%20%28single-precision%29) (DamageType :type Damage%20Type%20Object%20Reference) (InstigatedBy :type Controller%20Object%20Reference) (DamageCauser :type Actor%20Object%20Reference))
  (if (not (Math|Boolean|ORBoolean (Variables|Default|GetIs%20Invincible) (Variables|Default|GetIs%20Dashing) (Variables|Default|GetisDead)))
    (Development|PrintString "ouch")
    (Combat|DecreaseHealth)
    (Camera|PlayWorldCameraShake "/Game/Blueprints/HitShake.HitShake_C" (Transformation|GetActorLocation) 1e+03 1.5e+04 0.0 true)
    (if (<= (Variables|Default|Gethearts) 0)
      (Variables|Default|Sethearts 0)
      (Variables|Default|SetisDead true)
      (Animation|Montage|PlayMontage (Variables|Character|GetMesh) "/Game/ArtAssets/Temp/KidCharacter/Animations/Player_React_Death_Backward.Player_React_Death_Backward"
        (:then
          (Utilities|FlowControl|Delay 1.5)
          (Development|PrintString "Player: dead")
          ;[1 0 0.8489] Death UI
          (bind _returnvalue (UserInterface|CreateWidget "/Game/UI_Folder/HUD/Death_BP.Death_BP_C"))
          (UserInterface|Viewport|AddtoViewport _returnvalue 0)
          (Utilities|FlowControl|Delay 5.0)
          (Actor|DestroyActor)))
      (else
        ;[1 1 1] Temporary Invincibility Flash, Can Be Changed Later
        (Variables|Default|SetIs%20Invincible true)
        (bind _counter (Utilities|FlowControl|DoN 60)
          (:Exit
            (Utilities|FlowControl|FlipFlop
              (:A
                (Rendering|SetVisibility (Variables|Character|GetMesh) false false)
                (Utilities|FlowControl|Delay 0.1))
              (:B
                (Rendering|SetVisibility (Variables|Character|GetMesh) true false)
                (Utilities|FlowControl|Delay 0.1)))
            (Math|Integer|CompareInt _counter 25
              (:>
                (CallFunction|VisibilityChangeReset :!label _label)
                (Variables|Default|SetIs%20Invincible false)
                (Rendering|SetVisibility (Variables|Character|GetMesh) true false))
              (:==
                (goto _label))
              (:<
                (CallFunction|VisibilityChangeRepeat)))))))))

(event Input|ActionEvents|InputActionDash/Dodge
  (params (Key :type Key%20Structure :default "None"))
  (:Pressed
    (Variables|Default|SetIs%20Dashing true)
    (if (CharacterMovement|CheckCanDash)
      (Variables|PlayerMovement|SetcanDash/Dodge false)
      (Animation|Montage|PlayMontage (Variables|Character|GetMesh) "/Game/ArtAssets/Temp/KidCharacter/Animations/PlayerDodge.PlayerDodge" 1.5
        (:then
          (Pawn|SetControlRotation (Game|GetPlayerController 0) (CharacterMovement|FindRotationtoMovementAxis)))
        (:OnBlendOut
          (Variables|PlayerMovement|SetcanDash/Dodge true)
          (Variables|Default|SetIs%20Dashing false))))))

(event Input|ActionEvents|InputActionDash/DodgeController
  (params (Key :type Key%20Structure :default "None"))
  ;[0.9346 0 1] Controller Inputs
  ;;[1 0.03484 0.9213] Dash Controller
  (:Pressed
    (Variables|Default|SetIs%20Dashing true)
    (if (CharacterMovement|CheckCanDash)
      (Variables|PlayerMovement|SetcanDash/Dodge false)
      (Animation|Montage|PlayMontage (Variables|Character|GetMesh) "/Game/ArtAssets/Temp/KidCharacter/Animations/PlayerDodge.PlayerDodge" 1.5
        (:then
          (Pawn|SetControlRotation (Game|GetPlayerController 0) (CharacterMovement|FindRotationtoMovementAxis)))
        (:OnBlendOut
          (Variables|PlayerMovement|SetcanDash/Dodge true)
          (Variables|Default|SetIs%20Dashing false))))))

(event Input|ActionEvents|InputActionPause
  (params (Key :type Key%20Structure :default "None"))
  (bind _returnvalue (Game|GetPlayerController 0))
  ;[1 0 0.9839] Pause
  (:Pressed
    (Utilities|FlowControl|FlipFlop
      (:A
        (Game|SetGamePaused true)
        (bind _returnvalue_2 (UserInterface|CreateWidget "/Game/UI_Folder/Pause_Menu_Settings_Menu/Gameplay_BP.Gameplay_BP_C"))
        (UserInterface|Viewport|AddtoViewport _returnvalue_2 0)
        (Input|SetInputModeGameandUI _returnvalue 0 "DoNotLock" true)
        (Variables|/Script/Engine.PlayerController|SetbShowMouseCursor _returnvalue true))
      (:B
        (Game|SetGamePaused false)
        (Widget|RemovefromParent _returnvalue_2)
        (Input|SetInputModeGameOnly _returnvalue)
        (Variables|/Script/Engine.PlayerController|SetbShowMouseCursor _returnvalue false)))))

(event Input|ActionEvents|InputActionPauseController
  (params (Key :type Key%20Structure :default "None"))
  (bind _returnvalue (Game|GetPlayerController 0))
  ;[0.9346 0 1] Controller Inputs
  ;;[1 0.03484 0.9213] Controller Pause
  (:Pressed
    (Utilities|FlowControl|FlipFlop
      (:A
        (Game|SetGamePaused true)
        (bind _returnvalue_2 (UserInterface|CreateWidget "/Game/UI_Folder/Pause_Menu_Settings_Menu/Gameplay_BP.Gameplay_BP_C"))
        (UserInterface|Viewport|AddtoViewport _returnvalue_2 0)
        (bind _asgameplay_bp (Utilities|Casting|CastToGameplay_BP (Variables|Default|GetGameplaySettingsRef)))
        (Input|SetInputModeGameandUI _returnvalue (Variables|/Game/UI_Folder/Pause_Menu_Settings_Menu/Gameplay_BP.Gameplay_BP_C|GetResumebutton _asgameplay_bp) "DoNotLock" true)
        (Variables|/Script/Engine.PlayerController|SetbShowMouseCursor _returnvalue false))
      (:B
        (Game|SetGamePaused false)
        (Widget|RemovefromParent _returnvalue_2)
        (Input|SetInputModeGameOnly _returnvalue)
        (Variables|/Script/Engine.PlayerController|SetbShowMouseCursor _returnvalue false)))))

(event Input|ActionEvents|InputActionThrowStun
  (params (Key :type Key%20Structure :default "None"))
  ;[1 1 1] Throw stun -Z
  (:Pressed
    (if (!= (Variables|Default|GetStunCount) 0)
      (bind _result (Math|Integer|DecrementInt (Variables|Default|GetStunCount))
        (:%20%20
          (Variables|Default|SetStunCount _result)
          (bind _returnvalue (Game|SpawnActorfromClass "/Game/Blueprints/StunThrow/StunBP.StunBP_C" (Math|Transform|MakeTransform (Transformation|GetWorldLocation (Variables|Default|GetObjectRef)) (Transformation|GetWorldRotation (Variables|Collision|GetCapsuleComponent)) "1,1,1") "Undefined" 0 0))
          (Physics|SetPhysicsLinearVelocity (Variables|/Game/Blueprints/StunThrow/StunBP.StunBP_C|GetSphere%20collision _returnvalue) (* (Math|Vector|GetUnitDirection(Vector) (Transformation|GetActorLocation) (Transformation|GetActorLocation _returnvalue)) 5e+02) false "None"))))))

(event Input|ActionEvents|InputActionThrowStunController
  (params (Key :type Key%20Structure :default "None"))
  ;[0.9346 0 1] Controller Inputs
  ;;[1 0.03484 0.9213] Stun Controller
  (:Pressed
    (if (!= (Variables|Default|GetStunCount) 0)
      (bind _result (Math|Integer|DecrementInt (Variables|Default|GetStunCount))
        (:%20%20
          (Variables|Default|SetStunCount _result)
          (bind _returnvalue (Game|SpawnActorfromClass "/Game/Blueprints/StunThrow/StunBP.StunBP_C" (Math|Transform|MakeTransform (Transformation|GetWorldLocation (Variables|Default|GetObjectRef)) (Transformation|GetWorldRotation (Variables|Collision|GetCapsuleComponent)) "1,1,1") "Undefined" 0 0))
          (Physics|SetPhysicsLinearVelocity (Variables|/Game/Blueprints/StunThrow/StunBP.StunBP_C|GetSphere%20collision _returnvalue) (* (Math|Vector|GetUnitDirection(Vector) (Transformation|GetActorLocation) (Transformation|GetActorLocation _returnvalue)) 5e+02) false "None"))))))

(event Input|ActionEvents|InputActionLightAttack
  (params (Key :type Key%20Structure :default "None"))
  (:Pressed
    (if (CallFunction|CheckCanUseMoveInput)
      (Combat|InitiateAttack)))
  (:Released
    (if (CallFunction|CheckCanUseMoveInput)
      (Combat|Attack))))

(event Input|ActionEvents|InputActionLightAttackController
  (params (Key :type Key%20Structure :default "None"))
  ;[0.9346 0 1] Controller Inputs
  ;;[1 0.03484 0.9213] Light Attack Controller
  (:Pressed
    (if (CallFunction|CheckCanUseMoveInput)
      (Combat|InitiateAttack)))
  (:Released
    (if (CallFunction|CheckCanUseMoveInput)
      (Combat|Attack))))

(event Input|AxisEvents|InputAxisMoveRight/Left
  (params (AxisValue :type Float%20%28single-precision%29))
  (if (CallFunction|CheckCanUseMoveInput)
    (Pawn|Input|AddMovementInput "0.000000,1.000000, 0" AxisValue false)
    (Variables|PlayerMovement|SetmoveRight/LeftAxisValue AxisValue)))

(event Input|AxisEvents|InputAxisMoveForward/Backward
  (params (AxisValue :type Float%20%28single-precision%29))
  (if (CallFunction|CheckCanUseMoveInput)
    (Pawn|Input|AddMovementInput "1.000000, 0, 0" AxisValue false)
    (Variables|PlayerMovement|SetmoveForward/BackAxisValue AxisValue)))

(event Input|KeyboardEvents|AnyKey
  (params (Key :type Key%20Structure :default "None"))
  (:Pressed
    (Variables|Gamepad|SetisGamepadActive (Class|KismetInputLibrary|KeyIsGamepadKey Key))))

(event Input|KeyboardEvents|0
  (params (Key :type Key%20Structure :default "None"))
  ;[1 1 1] Debug for attached actors
  (:Pressed
    (for _array_element (Actor|GetAttachedActors true)
      (Development|PrintString (Utilities|GetDisplayName _array_element)))))

(event Input|KeyboardEvents|AnyKey
  (params (Key :type Key%20Structure :default "None"))
  ;[1 0 0.8217] Is gamepad active (for UI elements only)
  (:Pressed
    (if (Class|KismetInputLibrary|KeyIsGamepadKey Key)
      (Variables|Default|SetIs%20Using%20Gamepad?%20%28UI%29 true)
      (else
        (Variables|Default|SetIs%20Using%20Gamepad?%20%28UI%29 false)))))

(event Input|KeyboardEvents|E
  (params (Key :type Key%20Structure :default "None"))
  (:Pressed
    (Game|Damage|ApplyDamage self 5e+01 0 0)))

(fn ConstructionScript)

(fn ProcessCombat
  (if (Variables|Combat|GetisHoldingAttack)
    (Variables|Combat|SetattackHoldTime (+ (Utilities|Time|GetWorldDeltaSeconds) (Variables|Combat|GetattackHoldTime)))))

(fn InitiateAttack
  (if (not (Combat|CheckIsAttacking))
    (Variables|Combat|SetisHoldingAttack true)
    (Development|PrintString "Start Attack")))

(fn Attack
  (if (not (Combat|CheckIsAttacking))
    (Variables|Combat|SetisHoldingAttack false)
    (if (> (Variables|Combat|GetattackHoldTime) (Variables|Combat|GetholdTimeForHeavyAttack))
      (Combat|HeavyAttack)
      (else
        (Combat|LightAttack)))
    (Variables|Combat|SetattackHoldTime 0.0)))

(fn LightAttack
  (Development|PrintString "Player: LightAttack")
  (Animation|PlayAnimMontage "/Game/Characters/Janitor/NewLightAttack.NewLightAttack" 1.0 "None")
  (Default|ExecuteAttack (Variables|Default|GetCurrent%20weapon%20Actor)))

(fn HeavyAttack
  (Animation|PlayAnimMontage "/Game/Characters/Janitor/NewHeavyAttack.NewHeavyAttack" 1.0 "None")
  (Development|PrintString "Player: HeavyAttack")
  (for _array_element (Variables|Combat|GetenemiesInHitProximity)
    (if (Combat|CheckCanAttackEnemy _array_element)
      (Game|Damage|ApplyDamage _array_element 2e+01 0 0))))

(fn ProcessPlayerMovement
  (CharacterMovement|UpdatePlayerAim)
  (CallFunction|ProcessDodgeRoll))

(fn UpdatePlayerAim
  (if (CallFunction|CheckCanUseMoveInput)
    (if (Variables|Gamepad|GetisGamepadActive)
      (CharacterMovement|UpdateGamepadAim)
      (else
        (CharacterMovement|UpdateMouseAim)))))

(fn CheckThumbstickAboveDeadzone
  (return (> (Math|Vector2D|Vector2DLength (Math|Vector2D|MakeVector2D (Input|AxisValues|GetThumbstickAimUp/Down) (Input|AxisValues|GetThumbstickAimRight/Left))) (Variables|Gamepad|GetthumbstickDeadzoneSize))))

(fn GetMouseVelocity
  (bind _returnvalue (Game|GetPlayerController 0))
  (bind (_deltax _deltay) (Class|PlayerController|GetInputMouseDelta _returnvalue))
  (return (/ (Math|Vector2D|MakeVector2D _deltax _deltay) (Utilities|Time|GetWorldDeltaSeconds))))

(fn CheckMouseAboveDeadzone
  (return (> (Math|Vector2D|Vector2DLength (CharacterMovement|GetMouseVelocity)) (Variables|Keyboard&Mouse|GetmouseDeadzone))))

(fn UpdateMouseAim
  (bind _returnvalue (Game|GetPlayerController 0))
  (bind _returnvalue_2 (Game|GetPlayerController 0))
  (bind _hitresult (Game|Player|GetHitResultUnderCursorbyChannel _returnvalue "TraceTypeQuery1" true))
  (if (.bblockinghit _hitresult)
    (Variables|Default|SetMouseLocation (.location _hitresult))
    (Pawn|SetControlRotation _returnvalue_2 (Math|Interpolation|RInterpTo (Pawn|GetControlRotation _returnvalue_2 :!class /Script/Engine.Controller) (Math|Rotator|MakeRotator 0.0 0.0 (.yaw (Math|Rotator|FindLookatRotation (Transformation|GetActorLocation) (.location _hitresult)))) (Utilities|Time|GetWorldDeltaSeconds) (Variables|Keyboard&Mouse|GetmouseSmoothingStrength)))))

(fn UpdateGamepadAim
  (if (CharacterMovement|CheckThumbstickAboveDeadzone)
    (Pawn|SetControlRotation (Game|GetPlayerController 0) (Math|Rotator|MakeRotator 0.0 0.0 (Class|KismetMathLibrary|DegAtan2 (Input|AxisValues|GetThumbstickAimRight/Left) (Input|AxisValues|GetThumbstickAimUp/Down))))))

(fn DecreaseHealth
  (if (> (Variables|Default|GetTemporary%20Hearts) 0)
    (Math|Integer|DecrementInt (Variables|Default|GetTemporary%20Hearts)
      (:%20%20
        _))
    (else
      (Math|Integer|DecrementInt (Variables|Default|Gethearts)
        (:%20%20
          _))))
  (CallFunction|UpdateHearts)
  (return))

(fn GetIsAlive
  (return (not (Variables|Default|GetisDead))))

(fn GetDashDirection
  (return (Math|Vector2D|Normalize2D (Math|Vector2D|MakeVector2D (Variables|PlayerMovement|GetmoveForward/BackAxisValue) (Variables|PlayerMovement|GetmoveRight/LeftAxisValue)))))

(fn Dash
  (bind _dashstrength (Variables|PlayerMovement|GetdashStrength))
  (bind _dashdirection (CharacterMovement|GetDashDirection))
  (Physics|AddImpulse (Variables|Character|GetCharacterMovement) (Math|Vector|MakeVector (* (.x _dashdirection) _dashstrength) (* (.y _dashdirection) _dashstrength) 0.0) true)
  (Variables|PlayerMovement|SetcanDash/Dodge false))

(fn CheckCanDash
  (return (Math|Boolean|ANDBoolean (CallFunction|GetIsAlive) (Variables|PlayerMovement|GetcanDash/Dodge) (not (Variables|Default|GetisKnockedDown)))))

(fn CheckCanAttackEnemy
  (params (enemy :type Actor%20Object%20Reference))
  (bind _asbp_enemy (Utilities|Casting|CastToBP_Enemy enemy))
  (return (!= (Utilities|Array|FindItem (Variables|Combat|GetenemiesInHitProximity2) _asbp_enemy) -1)))

(fn CheckIsAttacking
  (return (Animation|Montage|MontageIsPlaying (Components|SkeletalMesh|GetAnimInstance (Variables|Character|GetMesh)) "/Game/Characters/Janitor/NewLightAttack.NewLightAttack")))

(fn FindRotationtoMovementAxis
  (bind _output_get (LocalVariables|SetlookAtLoc (+ (Transformation|GetActorLocation) (Math|Vector|MakeVector (Variables|PlayerMovement|GetmoveForward/BackAxisValue) (Variables|PlayerMovement|GetmoveRight/LeftAxisValue) 0.0))))
  (return (Math|Interpolation|RInterpTo (Pawn|GetControlRotation (Game|GetPlayerController 0) :!class /Script/Engine.Controller) (Math|Rotator|MakeRotator 0.0 0.0 (.yaw (Math|Rotator|FindLookatRotation (Transformation|GetActorLocation) _output_get))) (Utilities|Time|GetWorldDeltaSeconds) 0.0)))

(fn ProcessDodgeRoll
  (bind _moveright_leftaxisvalue (Variables|PlayerMovement|GetmoveRight/LeftAxisValue))
  (bind _moveforward_backaxisvalue (Variables|PlayerMovement|GetmoveForward/BackAxisValue))
  (bind _returnvalue (Math|Vector|MakeVector _moveforward_backaxisvalue _moveright_leftaxisvalue 0.0))
  (bind _returnvalue_2 (Math|Vector|Normalize _returnvalue))
  (if (and (not (Variables|Default|GetisKnockedDown)) (not (Variables|PlayerMovement|GetcanDash/Dodge)))
    (Pawn|Input|AddMovementInput (Math|Vector|MakeVector (.x _returnvalue_2) (.y _returnvalue_2) 0.0) 1.5 false)))

(fn CheckCanUseMoveInput
  (return (Math|Boolean|ANDBoolean (CallFunction|GetIsAlive) (Variables|PlayerMovement|GetcanDash/Dodge) (not (Variables|Default|GetisKnockedDown)))))

(fn CameraCollisionFunction
  (bind _outhits (Class|KismetSystemLibrary|BoxTraceMultiforObjects (Transformation|GetWorldLocation (Variables|Default|GetCamera%20Trace%20Start)) (Transformation|GetWorldLocation (Variables|Default|GetCamera)) "100.000000,200.000000,100.000000" "0, 0, 0" (Utilities|Array|MakeArray "ObjectTypeQuery1" "ObjectTypeQuery2") false (Collision|GetOverlappingActors (Variables|Default|GetBox) "/Game/Blueprints/MeshPlacer.MeshPlacer_C" :!class /Script/Engine.PrimitiveComponent) "None" true "(R=1.000000,G=0.000000,B=0.000000,A=1.000000)" "(R=0.000000,G=1.000000,B=0.000000,A=1.000000)" 1.0))
  (Utilities|Array|Clear (LocalVariables|GetCurrent%20Set))
  (for _array_element _outhits
    (bind _asmesh_placer (Utilities|Casting|CastToMeshPlacer (.HitActor (Collision|BreakHitResult _array_element))))
    (Utilities|Array|Add (LocalVariables|GetCurrent%20Set) _asmesh_placer))
  (for _array_element_2 (Variables|Default|GetCamera%20Object%20Overlaps)
    (if (not (Utilities|Array|ContainsItem (LocalVariables|GetCurrent%20Set) _array_element_2))
      (Default|VisibilityIncrease _array_element_2)))
  (for _array_element_3 (LocalVariables|GetCurrent%20Set)
    (if (not (Utilities|Array|ContainsItem (Variables|Default|GetCamera%20Object%20Overlaps) _array_element_3))
      (Default|VisibilityDecrease _array_element_3)))
  (Variables|Default|SetCamera%20Object%20Overlaps (LocalVariables|GetCurrent%20Set))
  (return))

(fn EquipWeapon
  (params (Weapon :type Actor%20Class%20Reference))
  (bind _mesh (Variables|Character|GetMesh))
  (bind _returnvalue (Game|SpawnActorfromClass Weapon (Transformation|GetSocketTransform _mesh "WeaponSocket" "RTS_World") "Undefined" 0 0))
  (bind _asbp_base_parent_weapon (Utilities|Casting|CastToBP_BaseParentWeapon _returnvalue))
  (Variables|Default|SetCurrent%20weapon%20Actor _asbp_base_parent_weapon)
  (Transformation|AttachComponentToComponent _returnvalue _mesh "WeaponSocket" "SnapToTarget" "SnapToTarget" "SnapToTarget" true))