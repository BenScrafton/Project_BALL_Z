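; MeshPlacer is a level-design actor that shows a configurable mesh and material and can fade its opacity out and back in.
; The construction script applies the chosen mesh and material, letting designers edit many placers at once, and tags the actor "Wall" when flagged.
; BeginPlay creates a dynamic material whose Opacity follows a timeline, played by VisibilityDecrease only when CanHide is set and reversed by VisibilityIncrease.
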(event Custom|Visibility%20Increase
  (if true
    (bind _visibility (Timeline|Timeline_0 ReverseFromEnd)
      (:Update
        (Rendering|Material|SetScalarParameterValue (Variables|Default|GetMaterial%20Reference) "Opacity" _visibility :!class /Script/Engine.MaterialInstanceDynamic)))))

(event Custom|Visibility%20Decrease
  (if (Variables|Default|GetCan%20Hide)
    (bind _visibility (Timeline|Timeline_0 PlayFromStart)
      (:Update
        (Rendering|Material|SetScalarParameterValue (Variables|Default|GetMaterial%20Reference) "Opacity" _visibility :!class /Script/Engine.MaterialInstanceDynamic)))))

(event EventBeginPlay
  (bind _mesh (Variables|Default|GetMesh))
  (bind _returnvalue (Rendering|Material|CreateDynamicMaterialInstance _mesh 0 (Rendering|Material|GetMaterial _mesh 0) "None" :!class /Script/Engine.PrimitiveComponent))
  (Variables|Default|SetMaterial%20Reference _returnvalue))

(fn ConstructionScript
  (bind _mesh (Variables|Default|GetMesh))
  ;[1 1 1] Allows level designers to change the mesh and material of multiple mesh placers at once
  (Components|StaticMesh|SetStaticMesh _mesh (Variables|Default|GetMesh%20To%20Use))
  (Rendering|Material|SetMaterial _mesh 0 (Variables|Default|GetMaterial%20To%20Use))
  (if (Variables|Default|GetIs%20A%20Wall)
    (Variables|Default|SetTags (Utilities|Array|MakeArray "Wall"))
    (else
      (Variables|Default|SetTags (Utilities|Array|MakeArray "None")))))