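; BP_CustomGravity is a component that applies simple vertical gravity to its owning actor.
; Each tick a downward sphere trace sets Grounded, either zeroing velocity and storing the hit location or calling Fall.
; Fall accumulates downward velocity from GravityStrength and moves the owner with a swept offset.
; OverrideGrounded skips the trace for a value settable through SetGrounded, though that branch falls when Grounded is true, which appears inverted.
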(event EventBeginPlay)

(event EventTick
  (params (DeltaSeconds :type Float%20%28single-precision%29))
  (if (Variables|Default|GetoverrideGrounded)
    (if (Variables|Default|Getgrounded)
      (CallFunction|Fall))
    (else
      (bind (_outhit _returnvalue) (Collision|SphereTraceByChannel (Transformation|GetActorLocation (Components|GetOwner)) (- (Transformation|GetActorLocation (Components|GetOwner)) (Math|Vector|MakeVector 0.0 0.0 (Variables|Default|GettraceLength))) 0.0 "TraceTypeQuery1" false 0 "None"))
      (if _returnvalue
        (Variables|Default|Setvelocity "0, 0, 0")
        (Variables|Default|Setgrounded true)
        (Variables|Default|SethitLocation (.location _outhit))
        (else
          (Variables|Default|Setgrounded false)
          (CallFunction|Fall))))))

(fn SetGrounded
  (params (grounded :type Boolean))
  (bind _output_get (Variables|Default|Setgrounded grounded))
  (if _output_get
    (Variables|Default|Setvelocity "0, 0, 0")))

(fn Fall
  (bind _output_get (Variables|Default|Setvelocity (Math|Vector|MakeVector 0.0 0.0 (+ (.z (Variables|Default|Getvelocity)) (* (* -1 (Variables|Default|GetGravityStrength)) (Utilities|Time|GetWorldDeltaSeconds))))))
  (Transformation|AddActorWorldOffset (Components|GetOwner) (Math|Vector|MakeVector 0.0 0.0 (* (.z _output_get) (Utilities|Time|GetWorldDeltaSeconds))) true))